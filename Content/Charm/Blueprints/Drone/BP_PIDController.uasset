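; BP_PIDController is a PID controller Blueprint in the Drone folder that turns an error value into a correction output.
; Its PIDController function sums proportional, integral and derivative terms from supplied gains and delta time, storing the integral and previous error between calls.
; The integral is unclamped, and the derivative low-pass filter is disconnected, so the FilterD input has no effect.
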(event EventBeginPlay)

(event EventTick
  (params (DeltaSeconds :type Float%20%28single-precision%29)))

(fn PIDController
  (params (Error :type Float%20%28double-precision%29) (Kp :type Float%20%28double-precision%29) (Ki :type Float%20%28double-precision%29) (Kd :type Float%20%28double-precision%29) (DeltaSecond :type Float%20%28double-precision%29) (FilterD :type Boolean))
  (Variables|Default|SetError Error)
  (Variables|Default|SetP (* Kp (Variables|Default|GetError))) ; Instant reaction to error
  (Variables|Default|SetI (+ (Variables|Default|GetI) (* Ki (Variables|Default|GetError) DeltaSecond)))
  (Variables|Default|SetD (* Kd (/ (- (Variables|Default|GetError) (Variables|Default|GetPreviousError)) DeltaSecond)))
  (Variables|Default|SetPreviousError (Variables|Default|GetError))
  (return (+ (Variables|Default|GetP) (Variables|Default|GetI) (Variables|Default|GetD))))