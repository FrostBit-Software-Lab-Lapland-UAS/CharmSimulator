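; Scenario event actor for a moving object, with a spline path that is editable at runtime using the mouse.
; Selection spawns BP_SplinePointIndicator handles and enables the Niagara spline visualizer; deselection clears both.
; Tick polls cursor traces: left-drag moves a handle and its spline point, Ctrl+click inserts one on the spline, mouse wheel nudges height.
; The base sphere represents point zero, so handle indices are offset by one.
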(event Custom|ShowSplinePoints
  (CallFunction|SpawnPointstoSpline)
  (Niagara|SetNiagaraVariable(Float) (Variables|Default|GetNS_SplineVisualizer) "SpawnRate" 2e+02))

(event Custom|RemoveSplinePoints
  (bind _arrayelement (Utilities|Array|ReverseforEachLoop (Variables|Default|GetSplinePoints))
    (:LoopBody
      (Actor|DestroyActor _arrayelement))
    (:Completed
      (Utilities|Array|Clear (Variables|Default|GetSplinePoints))
      (Niagara|SetNiagaraVariable(Float) (Variables|Default|GetNS_SplineVisualizer) "SpawnRate" 0.0))))

(event Custom|RemoveSplinePoint
  (bind _selectedsplinepoint (Variables|Default|GetSelectedSplinePoint))
  (bind _splinepoints (Variables|Default|GetSplinePoints))
  (bind _returnvalue (Utilities|Array|FindItem _splinepoints _selectedsplinepoint))
  (Spline|RemoveSplinePoint (Variables|Default|GetSpline) _returnvalue true)
  (Utilities|Array|RemoveIndex (Variables|Default|GetSplinePoints) _returnvalue)
  (Actor|DestroyActor (Variables|Default|GetSelectedSplinePoint)))

(event Custom|SetLoopClosed
  (params (isClosed :type Boolean))
  (Spline|SetClosedLoop (Variables|Default|GetSpline) isClosed true))

(event Custom|UpdateSplinePointLocationOnRoot
  (Spline|SetLocationatSplinePoint (Variables|Default|GetSpline) 0 (Transformation|GetActorLocation) "World" true))

(event EventBeginPlay
  (EventDispatchers|BindEventtoSelected (delegate Custom|ShowSplinePoints))
  (EventDispatchers|BindEventtoDeSelected (delegate Custom|RemoveSplinePoints))
  (EventDispatchers|BindEventtoZaxisUpdated (delegate Custom|UpdateSplinePointLocationOnRoot))
  (CallFunction|SpawnPointstoSpline)
  (Niagara|SetNiagaraVariable(Float) (Variables|Default|GetNS_SplineVisualizer) "SpawnRate" 2e+02))

(event EventTick
  (params (DeltaSeconds :type Float%20%28single-precision%29))
  (bind (_hitresult _returnvalue) (|GetHitResultUndeMouseIfConditionsAreMet))
  (bind (_returnvalue_2 _scrolledup) (|IsMouseWheelUsed))
  (bind (_bblockinghit _binitialoverlap _time _distance _location _impactpoint _normal _impactnormal _physmat _hitactor) (Collision|BreakHitResult _hitresult))
  (if _returnvalue
    (Utilities|Casting|CastToBP_ScenarioActor _hitactor
      (:then
        (Variables|Default|SetisMovingSplinePoint false)
        (Variables|Default|SetSelectedSplinePoint 0))
      (:CastFailed
        (if (|CTRLpressedorhold)
          (if (not (Variables|Default|GetisSplinePointAdded))
            (CallFunction|AddSplinePoint _impactpoint))
          (else
            (Variables|Default|SetisSplinePointAdded false)
            (bind _asbp_spline_point_indicator (Utilities|Casting|CastToBP_SplinePointIndicator _hitactor)
              (:then
                (Variables|Default|SetisMovingSplinePoint true)
                (if (!= _asbp_spline_point_indicator (Variables|Default|GetSelectedSplinePoint))
                  (Variables|Default|SetSelectedSplinePoint _asbp_spline_point_indicator) ; Select different spline point
                  (else
                    (CallFunction|MoveSinglePoint (CallFunction|GetSplinePointIndex) (+ (.ImpactPoint (Collision|BreakHitResult (.HitResult (Class|PlayerController|GetHitResultUnderCursorforObjects (Game|GetPlayerController 0) (Utilities|Array|MakeArray "ObjectTypeQuery9") true)))) (Math|Vector|MakeVector 0.0 0.0 2e+01)) :!label _label))))
              (:CastFailed
                (goto _label)))))))
    (elif _returnvalue_2
      (CallFunction|MoveSinglePoint (CallFunction|GetSplinePointIndex) (Math|Vector|MakeVector (.x (Transformation|GetActorLocation (Variables|Default|GetSelectedSplinePoint))) (.y (Transformation|GetActorLocation (Variables|Default|GetSelectedSplinePoint))) (+ (.z (Transformation|GetActorLocation (Variables|Default|GetSelectedSplinePoint))) (Math|Float|SelectFloat 1e+01 -1e+01 _scrolledup)))))))

(event EventEndPlay
  (params (EndPlayReason :type EEndPlayReason%20Enum :default "Destroyed"))
  (CallFunction|RemoveSplinePoints))

(fn ConstructionScript
  (|CallParentFunction))

(fn SpawnPointstoSpline
  (for _index (range 1 (- (Spline|GetNumberOfSplinePoints (Variables|Default|GetSpline)) 1)) ; Skip the first index because our sphere works as starting point
    (bind _returnvalue (Game|SpawnActorfromClass "/Game/Charm/Blueprints/TunnelGenerator/BP_SplinePointIndicator.BP_SplinePointIndicator_C" (Math|Transform|MakeTransform (Spline|GetLocationatSplinePoint (Variables|Default|GetSpline) _index "World") "0, 0, 0" "0.250000,0.250000,0.250000") "Undefined" 0 0))
    (Utilities|Array|Add (Variables|Default|GetSplinePoints) _returnvalue)
    (Transformation|AttachComponentToComponent _returnvalue (Variables|Default|GetBaseIndicatorMesh) "None" "KeepWorld" "KeepWorld" "KeepWorld" true)))

(fn MoveSinglePoint
  (params (Index :type Integer) (Location :type Vector))
  (Transformation|SetActorLocation (Variables|Default|GetSelectedSplinePoint) Location false false)
  (Spline|SetLocationatSplinePoint (Variables|Default|GetSpline) Index Location "World" true))

(fn GetSplinePointIndex
  (return (+ (Utilities|Array|FindItem (Variables|Default|GetSplinePoints) (Variables|Default|GetSelectedSplinePoint)) 1)))

(fn AddSplinePoint
  (params (WorldLocation :type Vector%20%28by%20ref%29))
  (bind _spline (Variables|Default|GetSpline))
  (bind _returnvalue (Spline|FindLocationClosesttoWorldLocation _spline WorldLocation "World"))
  (bind _output_get (LocalVariables|SetIndex (Math|Float|Ceil (Class|SplineComponent|FindInputKeyClosesttoWorldLocation _spline WorldLocation))))
  (Spline|AddSplinePointatIndex (Variables|Default|GetSpline) _returnvalue _output_get "World" true)
  (bind _returnvalue_2 (Game|SpawnActorfromClass "/Game/Charm/Blueprints/TunnelGenerator/BP_SplinePointIndicator.BP_SplinePointIndicator_C" (Math|Transform|MakeTransform _returnvalue "0, 0, 0" "0.250000,0.250000,0.250000") "Undefined" 0 0))
  (Utilities|Array|Insert (Variables|Default|GetSplinePoints) _returnvalue_2 (- (LocalVariables|GetIndex) 1))
  (Transformation|AttachComponentToComponent _returnvalue_2 (Variables|Default|GetBaseIndicatorMesh) "None" "KeepWorld" "KeepWorld" "KeepWorld" true)
  (Variables|Default|SetisSplinePointAdded true))