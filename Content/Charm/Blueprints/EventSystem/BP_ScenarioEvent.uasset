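; Scenario event Blueprint with test and reset hooks, plus a helper that picks spawn points for falling objects.
; TestEvent and ResetEvent both call TriggerEvent with opposite boolean flags, false for test and true for reset.
; The helper scales a random unit-cube offset by FallSpawnArea's world scale and adds its location, ignoring rotation.
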(event Custom|ResetEvent
  ;[0.06844 0 1 1 30] Test and reset
  (CallFunction|TriggerEvent true))

(event Custom|TestEvent
  ;[0.06844 0 1 1 30] Test and reset
  (CallFunction|TriggerEvent false))

(fn ConstructionScript)

(fn GetRandomPointforFallingObject0
  (bind _returnvalue (Math|Random|RandomFloatinRange -0.5 0.5))
  (bind _fallspawnarea (Variables|Default|GetFallSpawnArea))
  (bind _returnvalue_2 (Transformation|GetWorldTransform _fallspawnarea))
  (return (+ (* (Math|Vector|MakeVector (Math|Random|RandomFloatinRange -0.5 0.5) _returnvalue _returnvalue) (.scale _returnvalue_2)) (.location _returnvalue_2))))