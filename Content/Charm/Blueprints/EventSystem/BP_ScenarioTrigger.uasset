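; BP_ScenarioTrigger is a scenario trigger that fires when an inspection vehicle overlaps its indicator mesh in the simulation.
; On BeginPlay it colors the indicator orange and marks it selected through material parameters.
; On overlap it applies FrictionValue as the wheel friction multiplier on both back movement components, then calls TriggerEvent on every entry in ChainedEvents.
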(event OnComponentBeginOverlap(BaseIndicatorMesh)
  (params (OverlappedComponent :type Primitive%20Component%20Object%20Reference) (OtherActor :type Actor%20Object%20Reference) (OtherComp :type Primitive%20Component%20Object%20Reference) (OtherBodyIndex :type Integer) (bFromSweep :type Boolean) (SweepResult :type Hit%20Result%20Structure%20%28by%20ref%29))
  (bind _frictionvalue (Variables|Default|GetFrictionValue))
  ;[1 0.7641 0 1 30] This is the event when vehicle triggers scenario in simulation
  (bind _asbp_inspection_vechicle (Utilities|Casting|CastToBP_InspectionVechicle OtherActor))
  (Class|ChaosWheeledVehicleMovementComponent|SetWheelFrictionMultiplier (Variables|/Game/Charm/Blueprints/Vehicle/BP_InspectionVechicle.BP_InspectionVechicle_C|GetBackLeftMovementComponent _asbp_inspection_vechicle) 0 _frictionvalue)
  (Class|ChaosWheeledVehicleMovementComponent|SetWheelFrictionMultiplier (Variables|/Game/Charm/Blueprints/Vehicle/BP_InspectionVechicle.BP_InspectionVechicle_C|GetBackRightMovementComponent _asbp_inspection_vechicle) 0 _frictionvalue)
  (for _array_element (Variables|Default|GetChainedEvents)
    (Default|TriggerEvent _array_element false false)))

(event EventBeginPlay
  (bind _baseindicatormesh (Variables|Default|GetBaseIndicatorMesh))
  ;[1 0 0 1 30] Set trigger color
  (Rendering|Material|SetVectorParameterValueonMaterials _baseindicatormesh "Color" (Math|Vector|MakeVector 1.0 0.5 0.0))
  (Rendering|Material|SetScalarParameterValueonMaterials _baseindicatormesh "IsSelected" 1.0))

(fn ConstructionScript)