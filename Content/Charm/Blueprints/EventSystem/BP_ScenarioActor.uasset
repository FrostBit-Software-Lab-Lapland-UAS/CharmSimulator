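; Selectable scenario event actor that triggers falling props, moving objects or radar, lidar and camera failures.
; TriggerEvent waits a delay, runs its event type, then triggers ChainedEvents, which are destroyed on EndPlay.
; Falling props spawn randomly in the indicator mesh's box, retrying collision failures, and clear on reset.
; Failures pause sensor ticks, optionally timed, and skip test/reset; camera failure targets radar sensors, and moving objects only stores IsReset.
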(event Custom|TriggerEvent
  (params (isReset :type Boolean) (isTesting :type Boolean))
  (bind _returnvalue (or isReset isTesting))
  (bind _returnvalue_2 (not _returnvalue))
  ;[1 0.4169 0 1 30] If we are testing scenario isTest is first true and after all the events have been triggered we call trigger event again with isReset true.
  (if isReset
    _
    (else
      (Utilities|FlowControl|Delay (Variables|Default|GetDelay))))
  (switch Utilities|FlowControl|Switch|SwitchonScenarioEvents (Variables|Default|GetEventType)
    (:NewEnumerator0
      (CallFunction|FallEvent isReset)
      (for _array_element (Variables|Default|GetChainedEvents) :!label _label
        (CallFunction|TriggerEvent _array_element isReset isTesting)))
    (:NewEnumerator1
      (CallFunction|MovingObjectsEvent isReset)
      (goto _label))
    (:NewEnumerator3
      (if _returnvalue_2
        (CallFunction|RadarFailureEvent)
        (goto _label)))
    (:NewEnumerator4
      (if _returnvalue_2
        (CallFunction|LidarFailure)
        (goto _label)))
    (:NewEnumerator5
      (if _returnvalue_2
        (CallFunction|CameraFailure)
        (goto _label)))))

(event Custom|UpdateLocationOnZaxis
  (params (amount :type Float%20%28double-precision%29))
  (Transformation|AddActorLocalOffset (Math|Vector|MakeVector 0.0 0.0 amount) false false)
  (Default|CallZaxisUpdated))

(event Custom|CameraFailure
  ;[0 0.868 1 1 30] Camera failure event
  (bind _outactors (Actor|GetAllActorsOfClass "/Game/Charm/Blueprints/Sensors/BP_RadarSensor.BP_RadarSensor_C"))
  (for _array_element _outactors
    (Actor|Tick|SetActorTickEnabled _array_element))
  (if (!= (Variables|Default|GetSensorFailureTimer) 0.0)
    (Utilities|FlowControl|Delay (Variables|Default|GetSensorFailureTimer))
    (for _array_element_2 _outactors
      (Actor|Tick|SetActorTickEnabled _array_element_2 true))))

(event Custom|FallEvent
  (params (IsReset :type Boolean))
  (Variables|Default|SetisReset IsReset)
  (if (not IsReset)
    (for _index (range 1 (Variables|FallEvent|GetNumberOfFallingActors))
      (if (not (Variables|Default|GetisReset))
        (CallFunction|SpawnFallObject)))
    (if (> (Variables|FallEvent|GetNumberOfFallingActors) (Utilities|Array|Length (Variables|FallEvent|GetSpawnedFallActors))) :!label _label
      (Utilities|FlowControl|Delay 0.1)
      (for _index_2 (range 1 (- (Variables|FallEvent|GetNumberOfFallingActors) (Utilities|Array|Length (Variables|FallEvent|GetSpawnedFallActors))))
        (if (not (Variables|Default|GetisReset))
          (CallFunction|SpawnFallObject)))
      (goto _label))
    (else
      (bind _arrayelement (Utilities|Array|ReverseforEachLoop (Variables|FallEvent|GetSpawnedFallActors))
        (:LoopBody
          (Actor|DestroyActor _arrayelement))
        (:Completed
          (Utilities|Array|Clear (Variables|FallEvent|GetSpawnedFallActors)))))))

(event Custom|MovingObjectsEvent
  (params (isReset :type Boolean))
  ;[1 0.8883 0 1 30] Moving object event (dont remove)
  (Variables|Default|SetisReset isReset))

(event Custom|RadarFailureEvent
  ;[0.3853 1 0 1 30] Radar failure event
  (bind _outactors (Actor|GetAllActorsOfClass "/Game/Charm/Blueprints/Sensors/BP_RadarSensor.BP_RadarSensor_C"))
  (for _array_element _outactors
    (Actor|Tick|SetActorTickEnabled _array_element))
  (if (!= (Variables|Default|GetSensorFailureTimer) 0.0)
    (Utilities|FlowControl|Delay (Variables|Default|GetSensorFailureTimer))
    (for _array_element_2 _outactors
      (Actor|Tick|SetActorTickEnabled _array_element_2 true))))

(event Custom|Select
  ;[0.7296 0 1 1 30] Select and deselect active event
  (Rendering|Material|SetScalarParameterValueonMaterials (Variables|Default|GetBaseIndicatorMesh) "IsSelected" 1.0)
  (Variables|Default|SetisSelected true)
  (Default|CallSelected))

(event Custom|LidarFailure
  ;[0 1 0.3919 1 30] Lidar failure event
  (bind _outactors (Actor|GetAllActorsOfClass "/Game/Charm/Blueprints/Sensors/BP_LidarSensor.BP_LidarSensor_C"))
  (for _array_element _outactors
    (Actor|Tick|SetActorTickEnabled _array_element))
  (if (!= (Variables|Default|GetSensorFailureTimer) 0.0)
    (Utilities|FlowControl|Delay (Variables|Default|GetSensorFailureTimer))
    (for _array_element_2 _outactors
      (Actor|Tick|SetActorTickEnabled _array_element_2 true))))

(event Custom|DeSelect
  ;[0.7296 0 1 1 30] Select and deselect active event
  (Rendering|Material|SetScalarParameterValueonMaterials (Variables|Default|GetBaseIndicatorMesh) "IsSelected" 0.0)
  (Variables|Default|SetisSelected false)
  (Default|CallDeSelected))

(event EventEndPlay
  (params (EndPlayReason :type EEndPlayReason%20Enum :default "Destroyed"))
  ;[1 0 0.08283 1 30] When actor is removed from scene we remove all the chained events
  (for _array_element (Variables|Default|GetChainedEvents)
    (Actor|DestroyActor _array_element)))

(fn ConstructionScript)

(fn GetRandomPointforFallingObject
  (bind _baseindicatormesh (Variables|Default|GetBaseIndicatorMesh))
  (bind _returnvalue (Transformation|GetWorldScale _baseindicatormesh))
  (bind _returnvalue_2 (* _returnvalue 2e+02))
  (bind _returnvalue_3 (* _returnvalue_2 0.5))
  (return (Math|Random|RandomPointinBoundingBox (- (Transformation|GetWorldLocation _baseindicatormesh) (Math|Vector|MakeVector 0.0 0.0 (.z _returnvalue_3))) (Math|Vector|MakeVector (.x _returnvalue_3) (.y _returnvalue_3) (.z _returnvalue_3)))))

(fn SpawnFallObject
  (bind _returnvalue (CallFunction|GetRandomPointforFallingObject))
  (bind _returnvalue_2 (Game|SpawnActorfromClass "/Game/Charm/Blueprints/Props/BP_PropActor.BP_PropActor_C" (Math|Transform|MakeTransform _returnvalue (Math|Random|RandomRotator false) (Math|Vector|SelectVector (* "1.000000,1.000000,1.000000" (Math|Random|RandomFloatinRange 0.5 4.0)) "1.000000,1.000000,1.000000" (Utilities|Enum|Equal(Enum) (Variables|FallEvent|GetFallActorType) "NewEnumerator0"))) "DontSpawnIfColliding" 0 (select (Utilities|Enum|Equal(Enum) (Variables|FallEvent|GetFallActorType) "NewEnumerator6") (.OutItem (Utilities|Array|Random (Utilities|Array|MakeArray "NewEnumerator0" "NewEnumerator1" "NewEnumerator2" "NewEnumerator3"))) (Variables|FallEvent|GetFallActorType)) true 0))
  (Utilities|IsValid _returnvalue_2
    (:Is%20Valid
      (Utilities|Array|Add (Variables|FallEvent|GetSpawnedFallActors) _returnvalue_2))))