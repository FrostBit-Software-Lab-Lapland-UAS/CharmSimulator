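; Spline-driven procedural tunnel actor that works with the tunnel generator widget to be selected, edited and joined by intersections.
; ManualConstruction updates the spline and runs the generation loop, where C++-called events build one procedural mesh per segment with wall and ground sections.
; Point edits rebuild only nearby segments and refresh an end intersection if affected.
; An end indicator and overlap collider detect other tunnels, rejecting crossings between near-parallel tunnels.
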(event OnComponentBeginOverlap(ColliderTricker)
  (params (OverlappedComponent :type Primitive%20Component%20Object%20Reference) (OtherActor :type Actor%20Object%20Reference) (OtherComp :type Primitive%20Component%20Object%20Reference) (OtherBodyIndex :type Integer) (bFromSweep :type Boolean) (SweepResult :type Hit%20Result%20Structure%20%28by%20ref%29))
  (bind _tunnelgeneratorwidget (Variables|Default|GetTunnelGeneratorWidget))
  ;[1 0 0.914 1 30] When overlap sphere overlaps tunnel
  (if (not (Variables|Default|GetisEditingSplinePoints))
    (bind _asbp_procedural_tunnel (Utilities|Casting|CastToBP_ProceduralTunnel OtherActor))
    (if (Math|Boolean|ANDBoolean (== (Variables|Default|GetisSelected) 1.0) (> (Spline|GetSplineLength (Variables|Default|GetSplineComponent)) 1e+03) (> (Spline|GetSplineLength (Variables|/Script/CharmTunnelSim.ProceduralTunnel|GetSplineComponent _asbp_procedural_tunnel)) 2e+03) (|CollisionNotInStartOrEnd (Variables|/Script/CharmTunnelSim.ProceduralTunnel|GetSplineComponent _asbp_procedural_tunnel)))
      (if (or (.PointsEachOther (|AreEndsPointingEachOtherInOverlap (Variables|/Script/CharmTunnelSim.ProceduralTunnel|GetSplineComponent _asbp_procedural_tunnel))) (.PointsSameDirection (|AreEndsPointingEachOtherInOverlap (Variables|/Script/CharmTunnelSim.ProceduralTunnel|GetSplineComponent _asbp_procedural_tunnel))))
        (Rendering|Components|TextRender|SetText (Variables|/Game/Charm/HUDS/TunnelGenerator/WB_TunnelGenerate.WB_TunnelGenerate_C|Gettoast_text _tunnelgeneratorwidget) (select (.PointsEachOther (|AreEndsPointingEachOtherInOverlap (Variables|/Script/CharmTunnelSim.ProceduralTunnel|GetSplineComponent _asbp_procedural_tunnel))) "A crossing point cannot be added if the tunnels point towards each other." "A crossing point cannot be added if the tunnels point to same direction."))
        (UserInterface|Animation|PlayAnimation _tunnelgeneratorwidget (Variables|/Game/Charm/HUDS/TunnelGenerator/WB_TunnelGenerate.WB_TunnelGenerate_C|GetToast _tunnelgeneratorwidget) 0.0 1 "Forward" 1.0 false)
        (else
          (Default|SelectedOverlaps (Variables|Default|GetTunnelGeneratorWidget) _asbp_procedural_tunnel)))
      (Rendering|SetVisibility (Variables|Default|GetIndicator) false false))))

(event OnComponentEndOverlap(ColliderTricker)
  (params (OverlappedComponent :type Primitive%20Component%20Object%20Reference) (OtherActor :type Actor%20Object%20Reference) (OtherComp :type Primitive%20Component%20Object%20Reference) (OtherBodyIndex :type Integer))
  ;[1 0 0 1 30] When overlap ends
  (if (== (Variables|Default|GetisSelected) 1.0)
    (Default|SelectedStopOverlap (Variables|Default|GetTunnelGeneratorWidget))
    (Rendering|SetVisibility (Variables|Default|GetIndicator) true false)))

(event Custom|ManualConstruction
  (params (isSelected :type Float%20%28double-precision%29) (IsUndo :type Boolean) (TunnelScale :type Vector%202D%20Structure) (SurfaceVariation :type Vector%202D%20Structure) (Reset :type Boolean) (IsLoad :type Boolean) (IsPointAdjusted :type Boolean) (IsIntersectionAdded :type Boolean))
  (bind _tunneltype (Variables|Default|GettunnelType))
  (bind _splinepointindicator (Variables|Default|GetSplinePointIndicator))
  (bind _intersection (Variables|Default|GetIntersection))
  (bind _intersection_2 (Variables|Default|GetIntersection))
  ;[1 0 0.8317 1 30] ManualConstruction to update tunnel
  (Class|ProceduralTunnel|SetValues isSelected IsUndo TunnelScale SurfaceVariation Reset IsLoad)
  (if (Variables|Default|GetisLoad)
    (Collision|SetCollisionEnabled _splinepointindicator "NoCollision")
    (Rendering|SetVisibility _splinepointindicator false false))
  (Utilities|FlowControl|Sequence
    (:then_0
      (Class|ProceduralTunnel|SnaptoEndOfOtherSpline))
    (:then_1
      (Class|ProceduralTunnel|ControlSplinePoints IsIntersectionAdded))
    (:then_2
      (bind _returnvalue (Class|ProceduralTunnel|SetUpProceduralGeneratorLoopParams))
      (Utilities|IsValid _intersection_2
        (:Is%20Valid
          (Class|ProceduralTunnel|ProceduralGenerationLoop _returnvalue 0 false (Utilities|IsValid _intersection_2) (Variables|/Script/CharmTunnelSim.ProceduralIntersection|GetintersectionType _intersection_2)))
        (:Is%20Not%20Valid
          (Class|ProceduralTunnel|ProceduralGenerationLoop _returnvalue 0 false false "Right"))))
    (:then_3
      (if (not IsPointAdjusted)
        (if (and Reset (or (Utilities|Enum|Equal(Enum) _tunneltype "RightTunnel") (Utilities|Enum|Equal(Enum) _tunneltype "LeftTunnel")))
          (CallFunction|UpdateTunnelsNextto)
          (elif Reset
            (Utilities|IsValid _intersection
              (:Is%20Valid
                (Default|ManualConstruction _intersection (Variables|/Script/CharmTunnelSim.ProceduralIntersection|GetlocalScale _intersection) (Variables|/Script/CharmTunnelSim.ProceduralIntersection|GetintersectionType _intersection) self (Variables|/Script/CharmTunnelSim.ProceduralIntersection|GetsurfaceVariation _intersection) true)))))))))

(event Custom|ClearMeshComponents
  (bind _tunnelmeshes (Variables|Default|GetTunnelMeshes))
  ;[0.04267 0 1 1 30] For deleting
  (for _array_element _tunnelmeshes
    (Components|DestroyComponent _array_element))
  (Utilities|Array|Clear _tunnelmeshes))

(event Custom|ClearChildActors
  (bind _intersection (Variables|Default|GetIntersection))
  ;[0.04267 0 1 1 30] For deleting
  (Utilities|FlowControl|Sequence
    (:then_0
      (for _array_element (Actor|GetAttachedActors true false)
        (Actor|DestroyActor _array_element)))
    (:then_1
      (if (Utilities|IsValid _intersection)
        (Actor|DestroyActor _intersection)))))

(event Custom|Deselect
  ;[0.3765 1 0 1 30] Select/deselect tunel
  (for _array_element (Variables|Default|GetTunnelMeshes)
    (Rendering|Material|SetScalarParameterValueonMaterials _array_element "isSelected" 0.0)
    (Variables|Default|SetisSelected 0.0)))

(event Custom|Reselect
  ;[0.3765 1 0 1 30] Select/deselect tunel
  (for _array_element (Variables|Default|GetTunnelMeshes)
    (Rendering|Material|SetScalarParameterValueonMaterials _array_element "isSelected" 1.0)
    (Variables|Default|SetisSelected 1.0)))

(event EventEndPlay
  (params (EndPlayReason :type EEndPlayReason%20Enum :default "Destroyed"))
  (bind _intersection (Variables|Default|GetIntersection))
  ;[0.04267 0 1 1 30] For deleting
  (Utilities|FlowControl|Sequence
    (:then_0
      (for _array_element (Actor|GetAttachedActors true false)
        (Actor|DestroyActor _array_element)))
    (:then_1
      (if (Utilities|IsValid _intersection)
        (Actor|DestroyActor _intersection)))))

(event EventBeginPlay
  (bind _returnvalue (Actor|GetParentActor))
  (bind _splinecomponent (Variables|Default|GetSplineComponent))
  (bind _returnvalue_2 (Spline|GetNumberOfSplinePoints _splinecomponent))
  (bind _returnvalue_3 (- _returnvalue_2 1))
  (bind _returnvalue_4 (Spline|GetTransformatSplinePoint _splinecomponent _returnvalue_3 "World" false))
  ;[0 0.886 1 1 30] Beginplay
  (Transformation|SetWorldTransform (Variables|Default|GetSplinePointIndicator) (Math|Transform|MakeTransform (.location _returnvalue_4) (.rotation _returnvalue_4) "0.100000,0.100000,0.100000") false false)
  (bind _foundwidgets (Widget|GetAllWidgetsOfClass "/Game/Charm/HUDS/TunnelGenerator/WB_TunnelGenerate.WB_TunnelGenerate_C" true))
  (Variables|Default|SetTunnelGeneratorWidget (Utilities|Array|Get(acopy) _foundwidgets))
  (Utilities|IsValid _returnvalue
    (:Is%20Valid
      (bind _asbp_procedural_intersection (Utilities|Casting|CastToBP_ProceduralIntersection _returnvalue))
      (Variables|Default|SetPixelValues (Variables|/Game/Charm/Blueprints/TunnelGenerator/BP_ProceduralIntersection.BP_ProceduralIntersection_C|GetPixelValues _asbp_procedural_intersection)))))

(event EventMakeMeshTriangles
  (bind _pointsinheight (Variables|Default|GetpointsInHeight))
  ;[1 0 0.226 1 50] These functions are called from c++ from generating tunnel
  ;;[1 1 1 1 30] Create mesh triangles
  (bind _triangles (Class|KismetProceduralMeshLibrary|CreateGridMeshTriangles (+ (Variables|Default|GetpointCapLoopLastIndex) 1) (+ (Variables|Default|GetpointsInWidth) _pointsinheight _pointsinheight 1) false))
  (Variables|Default|SetwallTriangles _triangles)
  (bind _triangles_2 (Class|KismetProceduralMeshLibrary|CreateGridMeshTriangles (+ (Variables|Default|GetpointCapLoopLastIndex) 1) (+ (Variables|Default|GetpointsInWidth) 1) false))
  (Variables|Default|SetgroundTriangles _triangles_2))

(event EventTick
  (params (DeltaSeconds :type Float%20%28single-precision%29))
  (bind _indicator (Variables|Default|GetIndicator))
  (bind _splinecomponent (Variables|Default|GetSplineComponent))
  (bind _returnvalue (Spline|GetNumberOfSplinePoints _splinecomponent))
  (bind _returnvalue_2 (- _returnvalue 1))
  ;[1 0.1826 0 1 30] Move overlap indicator rock on tick
  (Transformation|SetWorldRotation _indicator (Math|Rotator|MakeRotator 0.0 0.0 (.yaw (Spline|GetRotationatSplinePoint _splinecomponent _returnvalue_2 "World"))) false false)
  (Transformation|SetWorldLocation _indicator (+ (* (Class|SplineComponent|GetDirectionatSplinePoint _splinecomponent _returnvalue_2 "World") (Math|Vector|MakeVector 6e+02 6e+02 6e+02)) (Spline|GetLocationatSplinePoint _splinecomponent _returnvalue_2 "World") (Math|Vector|MakeVector 0.0 0.0 3e+02)) false false)
  (Rendering|SetVisibility (Variables|Default|GetIndicator) (Math|Boolean|ANDBoolean (== (Variables|Default|GetisSelected) 1.0) (== (Variables|Default|GetisEndConnected) false) (== (Utilities|IsValid (Variables|Default|GetIntersection)) false)) false))

(event EventMakeMeshTangentsandNormals
  ;[1 0 0.226 1 50] These functions are called from c++ from generating tunnel
  ;;[1 1 1 1 30] Create normals and tangents
  (bind (_normals _tangents) (Class|KismetProceduralMeshLibrary|CalculateTangentsforMesh (Variables|Default|GetgroundVertices) (Variables|Default|GetgroundTriangles) (Variables|Default|GetgroundUV)))
  (Variables|Default|SetgroundNormals _normals)
  (Variables|Default|SetgroundTangents _tangents)
  (bind (_normals_2 _tangents_2) (Class|KismetProceduralMeshLibrary|CalculateTangentsforMesh (Variables|Default|GetwallVertices) (Variables|Default|GetwallTriangles) (Variables|Default|GetwallUV)))
  (Variables|Default|SetwallNormals _normals_2)
  (Variables|Default|SetwallTangents _tangents_2))

(event EventMakeMesh
  (params (meshIndex :type Integer) (isHeightChanged :type Boolean) (isFromLoad :type Boolean))
  (bind _isselected (Variables|Default|GetisSelected))
  (bind _recreatemeshcount (Variables|Default|GetreCreateMeshCount))
  (bind _splinecomponent (Variables|Default|GetSplineComponent))
  (bind _tunnelmeshes (Variables|Default|GetTunnelMeshes))
  (bind _returnvalue (Utilities|Array|Length _tunnelmeshes))
  (bind _returnvalue_2 (Spline|GetNumberOfSplinePoints _splinecomponent))
  (bind _returnvalue_3 (- _returnvalue_2 1))
  (bind _returnvalue_4 (- _returnvalue_3 _returnvalue))
  (bind _returnvalue_5 (!= _returnvalue_4 0))
  ;[1 0 0.226 1 50] These functions are called from c++ from generating tunnel
  ;;[1 1 1 1 30] Create meshes
  (if isHeightChanged
    (Class|ProceduralMeshComponent|CreateMeshSectionLinearColor (Utilities|Array|Get(acopy) (Variables|Default|GetTunnelMeshes) (Math|Integer|SelectInt (- (- (Utilities|Array|Length (Variables|Default|GetTunnelMeshes)) 1) meshIndex) (Variables|Default|GetmeshInRework) isHeightChanged)) 0 (Variables|Default|GetwallVertices) (Variables|Default|GetwallTriangles) (Variables|Default|GetwallNormals) (Variables|Default|GetwallUV) 0 0 0 0 (Variables|Default|GetwallTangents) true false :!label _label)
    (Class|ProceduralMeshComponent|CreateMeshSectionLinearColor (Utilities|Array|Get(acopy) (Variables|Default|GetTunnelMeshes) (Math|Integer|SelectInt (- (- (Utilities|Array|Length (Variables|Default|GetTunnelMeshes)) 1) meshIndex) (Variables|Default|GetmeshInRework) isHeightChanged)) 1 (Variables|Default|GetgroundVertices) (Variables|Default|GetgroundTriangles) (Variables|Default|GetgroundNormals) (Variables|Default|GetgroundUV) 0 0 0 0 (Variables|Default|GetgroundTangents) true false)
    (Rendering|Material|SetMaterial (Utilities|Array|Get(acopy) (Variables|Default|GetTunnelMeshes) (Math|Integer|SelectInt (- (- (Utilities|Array|Length (Variables|Default|GetTunnelMeshes)) 1) meshIndex) (Variables|Default|GetmeshInRework) isHeightChanged)) 0 "/Game/Charm/Materials/Tunnel/M_TunnelWall_Inst.M_TunnelWall_Inst")
    (Rendering|Material|SetMaterial (Utilities|Array|Get(acopy) (Variables|Default|GetTunnelMeshes) (Math|Integer|SelectInt (- (- (Utilities|Array|Length (Variables|Default|GetTunnelMeshes)) 1) meshIndex) (Variables|Default|GetmeshInRework) isHeightChanged)) 1 "/Game/Charm/Materials/Tunnel/M_TunnelGround_Inst.M_TunnelGround_Inst")
    (Utilities|Array|SetArrayElem (Variables|Default|GetmeshEnds) (Math|Integer|SelectInt (- (- (Utilities|Array|Length (Variables|Default|GetTunnelMeshes)) 1) meshIndex) (Variables|Default|GetmeshInRework) isHeightChanged) (Variables|Default|GetcurrentMeshEndData) true)
    (Rendering|Material|SetScalarParameterValueonMaterials (Utilities|Array|Get(acopy) (Variables|Default|GetTunnelMeshes) (Math|Integer|SelectInt (- (- (Utilities|Array|Length (Variables|Default|GetTunnelMeshes)) 1) meshIndex) (Variables|Default|GetmeshInRework) isHeightChanged)) "isSelected" _isselected)
    (Math|Integer|DecrementInt (Variables|Default|GetreCreateMeshCount))
    (else
      (if (not (or isFromLoad (Variables|Default|GetisReset)))
        (if (and (>= (Variables|Default|GetreCreateMeshCount) 0) (> (Utilities|Array|Length (Variables|Default|GetTunnelMeshes)) 0))
          (if (== (Variables|Default|GetmeshInRework) -1)
            (Variables|Default|SetmeshInRework (Math|Integer|Clamp(Integer) (- (Utilities|Array|LastIndex (Variables|Default|GetTunnelMeshes)) (Math|Integer|SelectInt (- _recreatemeshcount 1) _recreatemeshcount _returnvalue_5)) 0 999999))
            (else
              (Math|Integer|IncrementInt (Variables|Default|GetmeshInRework)
                (:%20%20
                  _))))
          (if (not (and (== (Variables|Default|GetreCreateMeshCount) 0) _returnvalue_5))
            (if (<= (Variables|Default|GetmeshInRework) (Utilities|Array|LastIndex (Variables|Default|GetTunnelMeshes)))
              (goto _label)
              (else
                _)))))
      (bind _returnvalue_6 (AddComponent|AddProceduralMeshComponent false (Math|Transform|MakeTransform "0, 0, 0")))
      (Utilities|Array|Add (Variables|Default|GetTunnelMeshes) _returnvalue_6)
      (Class|ProceduralMeshComponent|CreateMeshSectionLinearColor _returnvalue_6 0 (Variables|Default|GetwallVertices) (Variables|Default|GetwallTriangles) (Variables|Default|GetwallNormals) (Variables|Default|GetwallUV) 0 0 0 0 (Variables|Default|GetwallTangents) true false)
      (Class|ProceduralMeshComponent|CreateMeshSectionLinearColor _returnvalue_6 1 (Variables|Default|GetgroundVertices) (Variables|Default|GetgroundTriangles) (Variables|Default|GetgroundNormals) (Variables|Default|GetgroundUV) 0 0 0 0 (Variables|Default|GetgroundTangents) true false)
      (Rendering|Material|SetMaterial _returnvalue_6 0 "/Game/Charm/Materials/Tunnel/M_TunnelWall_Inst.M_TunnelWall_Inst")
      (Rendering|Material|SetMaterial _returnvalue_6 1 "/Game/Charm/Materials/Tunnel/M_TunnelGround_Inst.M_TunnelGround_Inst")
      (Rendering|Material|SetScalarParameterValueonMaterials _returnvalue_6 "isSelected" _isselected)
      (Utilities|Array|Add (Variables|Default|GetmeshEnds) (Variables|Default|GetcurrentMeshEndData)))))

(fn ConstructionScript)

(fn RemoveIntersection
  (bind _splinecomponent (Variables|Default|GetSplineComponent))
  (if (Utilities|IsValid (Variables|Default|GetIntersection))
    (Spline|SetSplinePointType _splinecomponent (- (Spline|GetNumberOfSplinePoints _splinecomponent) 1) "Curve" true)
    (Actor|DestroyActor (Variables|Default|GetIntersection))
    (Variables|Default|SetIntersection 0)
    (Utilities|Array|Clear (Variables|Default|GetmeshEndsBeforeIntersection))))

(fn AddIntersection
  (params (HasIntersection :type Boolean) (IntersectionType :type IntersectionType%20Enum :default "Right") (Scale :type Vector%202D%20Structure) (IntersectionAddedInMiddle :type Boolean))
  (bind _splinecomponent (Variables|Default|GetSplineComponent))
  (bind _returnvalue (Spline|GetSplineLength _splinecomponent))
  (bind _returnvalue_2 (Spline|GetTransformatDistanceAlongSpline _splinecomponent _returnvalue "World" false))
  (if (not HasIntersection) ; Boolean is true only when coming from load
    (if (> (Utilities|Array|Length (Variables|Default|GetmeshEndsBeforeIntersection)) 0)
      (if (Class|KismetMathLibrary|NotEqualExactlyVectorVector (Utilities|Array|Get(acopy) (.groundvertives (Utilities|Array|Get(acopy) (Variables|Default|GetmeshEnds)))) (Utilities|Array|Get(acopy) (.groundvertives (Utilities|Array|Get(acopy) (Variables|Default|GetmeshEndsBeforeIntersection)))))
        (Utilities|Array|Clear (Variables|Default|GetmeshEndsBeforeIntersection))
        (CallFunction|ManualConstruction 1.0 false (Variables|Default|GetlocalTunnelScale) (Variables|Default|GetsurfaceVariation) true false false false)))
    (if (== (Variables|Default|GetIntersectionIndex) 4)
      (CallFunction|RemoveIntersection)
      (Variables|Default|SetIntersectionIndex 0)
      (else
        (if IntersectionAddedInMiddle :!label _label
          (Variables|Default|SetIntersection 0)
          (Utilities|Array|Clear (Variables|Default|GetmeshEndsBeforeIntersection))
          (else
            (CallFunction|RemoveIntersection)))
        (Class|ProceduralTunnel|ProceduralGenerationLoop 0 0 true true (Utilities|Select :Index (Variables|Default|GetIntersectionIndex) :Option%200 "Right" :Option%201 "Left" :Option%202 "All" :Option%203 "RightLeft"))
        (bind _returnvalue_3 (Game|SpawnActorfromClass "/Game/Charm/Blueprints/TunnelGenerator/BP_ProceduralIntersection.BP_ProceduralIntersection_C" (Math|Transform|MakeTransform (.location _returnvalue_2) (.rotation _returnvalue_2) "1.000000,1.000000,1.000000") "AlwaysSpawn" 0 (Variables|Default|GetPixelValues) 0))
        (Transformation|AttachActorToActor _returnvalue_3 self "None" "KeepWorld" "KeepWorld" "KeepWorld" true)
        (Default|ManualConstruction _returnvalue_3 Scale (Utilities|Select :Index (Variables|Default|GetIntersectionIndex) :Option%200 "Right" :Option%201 "Left" :Option%202 "All" :Option%203 "RightLeft") self (Variables|Default|GetsurfaceVariation) false)
        (Variables|Default|SetIntersection _returnvalue_3)
        (Math|Integer|IncrementInt (Variables|Default|GetIntersectionIndex)
          (:%20%20
            (Variables|Default|SetmeshEndsBeforeIntersection (Variables|Default|GetmeshEnds))
            (return _returnvalue_3)))))
    (else
      (Variables|Default|SetIntersectionIndex (Utilities|Select :Index IntersectionType :Option%200 0 :Option%201 1 :Option%202 2 :Option%203 3))
      (goto _label))))

(fn CreateDisplacementTexture
  (bind _walldeformrendertarget (Variables|Default|GetwallDeformRenderTarget))
  (bind _returnvalue (Rendering|Material|CreateDynamicMaterialInstance "/Game/Charm/Materials/Tunnel/M_TunnelNoise.M_TunnelNoise" "None" "None" :!class /Script/Engine.KismetMaterialLibrary))
  (Rendering|Material|SetScalarParameterValue _returnvalue "NoiseScale" (Math|Random|RandomFloatinRange 0.1 1.0) :!class /Script/Engine.MaterialInstanceDynamic)
  (Rendering|DrawMaterialtoRenderTarget _walldeformrendertarget _returnvalue)
  (bind _outsamples (Class|KismetRenderingLibrary|ReadRenderTarget _walldeformrendertarget true))
  (Variables|Default|SetPixelValues _outsamples))

(fn UpdateSplinePointMovement
  (params (PointIndex :type Array%20of%20Integers))
  (bind _tunnelmeshes (Variables|Default|GetTunnelMeshes))
  (bind _intersection (Variables|Default|GetIntersection))
  (bind _intersection_2 (Variables|Default|GetIntersection))
  (bind _returnvalue (Utilities|Array|Length _tunnelmeshes))
  (bind _returnvalue_2 (- _returnvalue 1))
  (LocalVariables|SetbUpdateIntersection false)
  (for _array_element PointIndex
    (Utilities|IsValid (Variables|Default|GetIntersection)
      (:Is%20Valid
        (if (>= _array_element (- (Spline|GetNumberOfSplinePoints (Variables|Default|GetSplineComponent)) 2))
          (Class|ProceduralTunnel|ProceduralGenerationLoop (* (Math|Integer|Clamp(Integer) (- _returnvalue_2 (- _array_element 2)) 0 _returnvalue_2) -1) (* (Math|Integer|Clamp(Integer) (- _returnvalue_2 (+ _array_element 2)) 0 _returnvalue_2) -1) true (and (== (* (Math|Integer|Clamp(Integer) (- _returnvalue_2 (+ _array_element 2)) 0 _returnvalue_2) -1) 0) (Utilities|IsValid _intersection_2)) (Variables|/Script/CharmTunnelSim.ProceduralIntersection|GetintersectionType _intersection_2))
          (LocalVariables|SetbUpdateIntersection true)
          (else
            (Class|ProceduralTunnel|ProceduralGenerationLoop (* (Math|Integer|Clamp(Integer) (- _returnvalue_2 (- _array_element 2)) 0 _returnvalue_2) -1) (* (Math|Integer|Clamp(Integer) (- _returnvalue_2 (+ _array_element 2)) 0 _returnvalue_2) -1) true false "Right" :!label _label))))
      (:Is%20Not%20Valid
        (goto _label))))
  (if (LocalVariables|GetbUpdateIntersection)
    (Utilities|IsValid _intersection
      (:Is%20Valid
        (Default|ManualConstruction _intersection (Variables|/Script/CharmTunnelSim.ProceduralIntersection|GetlocalScale _intersection) (Variables|/Script/CharmTunnelSim.ProceduralIntersection|GetintersectionType _intersection) self (Variables|/Script/CharmTunnelSim.ProceduralIntersection|GetsurfaceVariation _intersection) true)))))

(fn GetPixelValue
  (params (x :type Integer) (y :type Integer))
  (return (.r (Math|Conversions|ToLinearColor(Color) (Utilities|Array|Get(acopy) (Variables|Default|GetPixelValues) (+ (- y 1) (* x (+ (* (Variables|Default|GetpointsInHeight) 2) (* (Variables|Default|GetpointsInWidth) 2) (Variables|Default|GetsplineLoopAdjustment)))))))))

(fn UpdateTunnelsNextto
  (bind _rightsidetunnel (Variables|Default|GetrightSideTunnel))
  (bind _leftsidetunnel (Variables|Default|GetleftSideTunnel))
  (bind _tunnelmeshes (Variables|/Script/CharmTunnelSim.ProceduralTunnel|GetTunnelMeshes _rightsidetunnel))
  (bind _tunnelmeshes_2 (Variables|/Script/CharmTunnelSim.ProceduralTunnel|GetTunnelMeshes _leftsidetunnel))
  (bind _returnvalue (Utilities|Array|Length _tunnelmeshes))
  (bind _returnvalue_2 (Utilities|Array|Length _tunnelmeshes_2))
  (bind _returnvalue_3 (- _returnvalue 1))
  (bind _returnvalue_4 (- _returnvalue_2 1))
  (bind _returnvalue_5 (* _returnvalue_3 -1))
  (bind _returnvalue_6 (* _returnvalue_4 -1))
  (Utilities|FlowControl|Sequence
    (:then_0
      (Utilities|IsValid _rightsidetunnel
        (:Is%20Valid
          (Class|ProceduralTunnel|ProceduralGenerationLoop _rightsidetunnel _returnvalue_5 _returnvalue_5 true false "Right"))))
    (:then_1
      (Utilities|IsValid _leftsidetunnel
        (:Is%20Valid
          (Class|ProceduralTunnel|ProceduralGenerationLoop _leftsidetunnel _returnvalue_6 _returnvalue_6 true false "Right"))))))