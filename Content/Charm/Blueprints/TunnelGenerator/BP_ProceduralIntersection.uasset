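; Procedural intersection actor for a tunnel generator, joining a parent tunnel to right, left and/or straight branches by intersection type.
; It builds wall and ground grids as two procedural mesh sections with computed normals, tangents and collision.
; It spawns BP_ProceduralTunnel child actors at the exits, shares point counts, links neighbouring tunnels and triggers their construction.
; On updates, it regenerates part of the existing left and right tunnels and refreshes their neighbours.
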(event Custom|ManualConstruction
  (params (Scale :type Vector%202D%20Structure) (Selection :type IntersectionType%20Enum :default "Right") (Parent :type Procedural%20Tunnel%20Object%20Reference) (SurfaceVariation :type Vector%202D%20Structure) (isUpdate :type Boolean))
  (bind _righttunnel (Variables|Default|GetRightTunnel))
  (bind _lefttunnel (Variables|Default|GetLeftTunnel))
  (bind _tunnelmeshes (Variables|/Script/CharmTunnelSim.ProceduralTunnel|GetTunnelMeshes _righttunnel))
  (bind _tunnelmeshes_2 (Variables|/Script/CharmTunnelSim.ProceduralTunnel|GetTunnelMeshes _lefttunnel))
  (bind _returnvalue (Utilities|Array|Length _tunnelmeshes))
  (bind _returnvalue_2 (Utilities|Array|Length _tunnelmeshes_2))
  (bind _returnvalue_3 (- _returnvalue 1))
  (bind _returnvalue_4 (- _returnvalue_2 1))
  (bind _returnvalue_5 (* _returnvalue_3 -1))
  (bind _returnvalue_6 (* _returnvalue_4 -1))
  (Class|ProceduralIntersection|SetValues Scale Selection Parent SurfaceVariation isUpdate)
  (Class|ProceduralIntersection|ClearArrays)
  (Class|ProceduralIntersection|IntersectionGenerationLoop)
  (if isUpdate
    (Utilities|FlowControl|Sequence
      (:then_0
        (Utilities|IsValid _lefttunnel
          (:Is%20Valid
            (Class|ProceduralTunnel|ProceduralGenerationLoop _lefttunnel _returnvalue_6 _returnvalue_6 true false)
            (Default|UpdateTunnelsNextto _lefttunnel))))
      (:then_1
        (Utilities|IsValid _righttunnel
          (:Is%20Valid
            (Class|ProceduralTunnel|ProceduralGenerationLoop _righttunnel _returnvalue_5 _returnvalue_5 true false)
            (Default|UpdateTunnelsNextto _righttunnel)))))))

(event Custom|CustomEventASD
  (bind _straighttunnel (Variables|Default|GetStraightTunnel))
  (bind _straighttunnel_2 (Variables|Default|GetStraightTunnel))
  (bind _straighttunnel_3 (Variables|Default|GetStraightTunnel))
  (bind _lefttunnel (Variables|Default|GetLeftTunnel))
  (bind _righttunnel (Variables|Default|GetRightTunnel))
  (switch Utilities|FlowControl|Switch|SwitchonIntersectionType (Variables|Default|GetintersectionType)
    (:Right
      (Utilities|FlowControl|Sequence
        (:then_0
          (|CreateRightTunnel_2 :!label _label))
        (:then_1
          (|CreateStraightTunnel_2 :!label _label_2))
        (:then_2
          (Variables|/Script/CharmTunnelSim.ProceduralTunnel|SetrightSideTunnel _straighttunnel_2 _righttunnel)
          (Variables|/Script/CharmTunnelSim.ProceduralTunnel|SetleftSideTunnel _righttunnel _straighttunnel_2)
          (Default|ManualConstruction (Variables|Default|GetRightTunnel) 0.0 false (Variables|Default|GetlocalScale) (Variables|Default|GetsurfaceVariation) false false false false)
          (Default|ManualConstruction (Variables|Default|GetStraightTunnel) 0.0 false (Variables|Default|GetlocalScale) (Variables|Default|GetsurfaceVariation) false false false false))))
    (:Left
      (Utilities|FlowControl|Sequence
        (:then_0
          (|CreateLeftTunnel_2 :!label _label_3))
        (:then_1
          (goto _label_2))
        (:then_2
          (Variables|/Script/CharmTunnelSim.ProceduralTunnel|SetleftSideTunnel _straighttunnel_3 _lefttunnel)
          (Variables|/Script/CharmTunnelSim.ProceduralTunnel|SetrightSideTunnel _lefttunnel _straighttunnel_3)
          (Default|ManualConstruction (Variables|Default|GetLeftTunnel) 0.0 false (Variables|Default|GetlocalScale) (Variables|Default|GetsurfaceVariation) false false false false)
          (Default|ManualConstruction (Variables|Default|GetStraightTunnel) 0.0 false (Variables|Default|GetlocalScale) (Variables|Default|GetsurfaceVariation) false false false false))))
    (:All
      (Utilities|FlowControl|Sequence
        (:then_0
          (goto _label))
        (:then_1
          (goto _label_3))
        (:then_2
          (goto _label_2))
        (:then_3
          (Variables|/Script/CharmTunnelSim.ProceduralTunnel|SetleftSideTunnel _straighttunnel (Variables|Default|GetLeftTunnel))
          (Variables|/Script/CharmTunnelSim.ProceduralTunnel|SetrightSideTunnel _straighttunnel (Variables|Default|GetRightTunnel))
          (Variables|/Script/CharmTunnelSim.ProceduralTunnel|SetrightSideTunnel (Variables|Default|GetLeftTunnel) _straighttunnel)
          (Variables|/Script/CharmTunnelSim.ProceduralTunnel|SetleftSideTunnel (Variables|Default|GetRightTunnel) _straighttunnel)
          (Default|ManualConstruction (Variables|Default|GetLeftTunnel) 0.0 false (Variables|Default|GetlocalScale) (Variables|Default|GetsurfaceVariation) false false false false)
          (Default|ManualConstruction (Variables|Default|GetRightTunnel) 0.0 false (Variables|Default|GetlocalScale) (Variables|Default|GetsurfaceVariation) false false false false)
          (Default|ManualConstruction (Variables|Default|GetStraightTunnel) 0.0 false (Variables|Default|GetlocalScale) (Variables|Default|GetsurfaceVariation) false false false false))))
    (:RightLeft
      (Utilities|FlowControl|Sequence
        (:then_0
          (goto _label))
        (:then_1
          (goto _label_3))
        (:then_2
          (Default|ManualConstruction (Variables|Default|GetRightTunnel) 0.0 false (Variables|Default|GetlocalScale) (Variables|Default|GetsurfaceVariation) false false false false)
          (Default|ManualConstruction (Variables|Default|GetLeftTunnel) 0.0 false (Variables|Default|GetlocalScale) (Variables|Default|GetsurfaceVariation) false false false false))))))

(event EventBeginPlay)

(event EventMakeMeshTriangles
  (bind _numberofhorizontalpoints (Variables|Default|GetnumberOfHorizontalPoints))
  (bind _numberofhorizontalpoints_2 (Variables|Default|GetnumberOfHorizontalPoints))
  (bind _numberofhorizontalpoints_3 (Variables|Default|GetnumberOfHorizontalPoints))
  (bind _numberofhorizontalpoints_4 (Variables|Default|GetnumberOfHorizontalPoints))
  (bind _numberofhorizontalpoints_5 (Variables|Default|GetnumberOfHorizontalPoints))
  (bind _numberofhorizontalpoints_6 (Variables|Default|GetnumberOfHorizontalPoints))
  (switch Utilities|FlowControl|Switch|SwitchonIntersectionType (Variables|Default|GetintersectionType)
    (:Right
      (bind _triangles (Class|KismetProceduralMeshLibrary|CreateGridMeshTriangles (Variables|Default|GetnumberOfHorizontalPoints) (+ (Variables|Default|GetnumberOfHorizontalPoints) (Variables|Default|GetnumberOfVerticalPoints)) false))
      (Variables|Default|SetTriangles _triangles)
      (bind _triangles_2 (Class|KismetProceduralMeshLibrary|CreateGridMeshTriangles _numberofhorizontalpoints_6 _numberofhorizontalpoints_6 false))
      (Variables|Default|SetGroundTriangles _triangles_2))
    (:Left
      (bind _triangles_3 (Class|KismetProceduralMeshLibrary|CreateGridMeshTriangles _numberofhorizontalpoints (+ _numberofhorizontalpoints (Variables|Default|GetnumberOfVerticalPoints)) false))
      (Variables|Default|SetTriangles _triangles_3)
      (bind _triangles_4 (Class|KismetProceduralMeshLibrary|CreateGridMeshTriangles _numberofhorizontalpoints_5 _numberofhorizontalpoints_5 false))
      (Variables|Default|SetGroundTriangles _triangles_4))
    (:All
      (bind _triangles_5 (Class|KismetProceduralMeshLibrary|CreateGridMeshTriangles _numberofhorizontalpoints_2 _numberofhorizontalpoints_2 false))
      (Variables|Default|SetTriangles _triangles_5)
      (bind _triangles_6 (Class|KismetProceduralMeshLibrary|CreateGridMeshTriangles _numberofhorizontalpoints_3 _numberofhorizontalpoints_3 false))
      (Variables|Default|SetGroundTriangles _triangles_6))
    (:RightLeft
      (bind _triangles_7 (Class|KismetProceduralMeshLibrary|CreateGridMeshTriangles (+ (Variables|Default|GetnumberOfHorizontalPoints) (Variables|Default|GetnumberOfVerticalPoints)) (Variables|Default|GetnumberOfHorizontalPoints) false))
      (Variables|Default|SetTriangles _triangles_7)
      (bind _triangles_8 (Class|KismetProceduralMeshLibrary|CreateGridMeshTriangles _numberofhorizontalpoints_4 _numberofhorizontalpoints_4 false))
      (Variables|Default|SetGroundTriangles _triangles_8))))

(event EventMakeMeshTangentsandNormals
  (bind (_normals _tangents) (Class|KismetProceduralMeshLibrary|CalculateTangentsforMesh (Variables|Default|GetwallVertices) (Variables|Default|GetTriangles)))
  (Variables|Default|SetNormals _normals)
  (Variables|Default|SetTangents _tangents)
  (bind (_normals_2 _tangents_2) (Class|KismetProceduralMeshLibrary|CalculateTangentsforMesh (Variables|Default|GetgroundVertices) (Variables|Default|GetGroundTriangles)))
  (Variables|Default|SetGroundNormals _normals_2)
  (Variables|Default|SetGroundTangents _tangents_2))

(event EventMakeMesh
  (bind _proceduralmesh (Variables|Default|GetProceduralMesh))
  (Class|ProceduralMeshComponent|CreateMeshSectionLinearColor _proceduralmesh 0 (Variables|Default|GetwallVertices) (Variables|Default|GetTriangles) (Variables|Default|GetNormals) 0 0 0 0 0 (Variables|Default|GetTangents) true false)
  (Class|ProceduralMeshComponent|CreateMeshSectionLinearColor _proceduralmesh 1 (Variables|Default|GetgroundVertices) (Variables|Default|GetGroundTriangles) (Variables|Default|GetGroundNormals) 0 0 0 0 0 (Variables|Default|GetGroundTangents) true false)
  (Rendering|Material|SetMaterial _proceduralmesh 0 "/Game/Charm/Materials/Tunnel/Wall/M_TunnelWall_Inst.M_TunnelWall_Inst")
  (Rendering|Material|SetMaterial _proceduralmesh 1 "/Game/Charm/Materials/Tunnel/Ground/M_TunnelGround_Inst.M_TunnelGround_Inst"))

(event EventAddContinuationTunnels
  (bind _straighttunnel (Variables|Default|GetStraightTunnel))
  (bind _straighttunnel_2 (Variables|Default|GetStraightTunnel))
  (bind _straighttunnel_3 (Variables|Default|GetStraightTunnel))
  (bind _lefttunnel (Variables|Default|GetLeftTunnel))
  (bind _righttunnel (Variables|Default|GetRightTunnel))
  (switch Utilities|FlowControl|Switch|SwitchonIntersectionType (Variables|Default|GetintersectionType)
    (:Right
      (Utilities|FlowControl|Sequence
        (:then_0
          (|CreateRightTunnel_2 :!label _label))
        (:then_1
          (|CreateStraightTunnel_2 :!label _label_2))
        (:then_2
          (Variables|/Script/CharmTunnelSim.ProceduralTunnel|SetrightSideTunnel _straighttunnel_2 _righttunnel)
          (Variables|/Script/CharmTunnelSim.ProceduralTunnel|SetleftSideTunnel _righttunnel _straighttunnel_2)
          (Default|ManualConstruction (Variables|Default|GetRightTunnel) 0.0 false (Variables|Default|GetlocalScale) (Variables|Default|GetsurfaceVariation) false false false false)
          (Default|ManualConstruction (Variables|Default|GetStraightTunnel) 0.0 false (Variables|Default|GetlocalScale) (Variables|Default|GetsurfaceVariation) false false false false))))
    (:Left
      (Utilities|FlowControl|Sequence
        (:then_0
          (|CreateLeftTunnel_2 :!label _label_3))
        (:then_1
          (goto _label_2))
        (:then_2
          (Variables|/Script/CharmTunnelSim.ProceduralTunnel|SetleftSideTunnel _straighttunnel_3 _lefttunnel)
          (Variables|/Script/CharmTunnelSim.ProceduralTunnel|SetrightSideTunnel _lefttunnel _straighttunnel_3)
          (Default|ManualConstruction (Variables|Default|GetLeftTunnel) 0.0 false (Variables|Default|GetlocalScale) (Variables|Default|GetsurfaceVariation) false false false false)
          (Default|ManualConstruction (Variables|Default|GetStraightTunnel) 0.0 false (Variables|Default|GetlocalScale) (Variables|Default|GetsurfaceVariation) false false false false))))
    (:All
      (Utilities|FlowControl|Sequence
        (:then_0
          (goto _label))
        (:then_1
          (goto _label_3))
        (:then_2
          (goto _label_2))
        (:then_3
          (Variables|/Script/CharmTunnelSim.ProceduralTunnel|SetleftSideTunnel _straighttunnel (Variables|Default|GetLeftTunnel))
          (Variables|/Script/CharmTunnelSim.ProceduralTunnel|SetrightSideTunnel _straighttunnel (Variables|Default|GetRightTunnel))
          (Variables|/Script/CharmTunnelSim.ProceduralTunnel|SetrightSideTunnel (Variables|Default|GetLeftTunnel) _straighttunnel)
          (Variables|/Script/CharmTunnelSim.ProceduralTunnel|SetleftSideTunnel (Variables|Default|GetRightTunnel) _straighttunnel)
          (Default|ManualConstruction (Variables|Default|GetLeftTunnel) 0.0 false (Variables|Default|GetlocalScale) (Variables|Default|GetsurfaceVariation) false false false false)
          (Default|ManualConstruction (Variables|Default|GetRightTunnel) 0.0 false (Variables|Default|GetlocalScale) (Variables|Default|GetsurfaceVariation) false false false false)
          (Default|ManualConstruction (Variables|Default|GetStraightTunnel) 0.0 false (Variables|Default|GetlocalScale) (Variables|Default|GetsurfaceVariation) false false false false))))
    (:RightLeft
      (Utilities|FlowControl|Sequence
        (:then_0
          (goto _label))
        (:then_1
          (goto _label_3))
        (:then_2
          (Default|ManualConstruction (Variables|Default|GetRightTunnel) 0.0 false (Variables|Default|GetlocalScale) (Variables|Default|GetsurfaceVariation) false false false false)
          (Default|ManualConstruction (Variables|Default|GetLeftTunnel) 0.0 false (Variables|Default|GetlocalScale) (Variables|Default|GetsurfaceVariation) false false false false))))))

(fn ConstructionScript)

(fn GetPixelValue
  (params (x :type Integer) (y :type Integer))
  (return (.r (Math|Conversions|ToLinearColor(Color) (Utilities|Array|Get(acopy) (Variables|Default|GetPixelValues) (+ y (* x (+ (* (Variables|Default|GetnumberOfVerticalPoints) 2) (* (Variables|Default|GetnumberOfHorizontalPoints) 2)))))))))

(fn SetChildPointValues
  (params (NewParam :type BP%20Procedural%20Tunnel%20Object%20Reference))
  (Utilities|FlowControl|Sequence
    (:then_0
      (Variables|/Script/CharmTunnelSim.ProceduralTunnel|SetnumberOfHorizontalPoints NewParam (Variables|Default|GetnumberOfHorizontalPoints)))
    (:then_1
      (Variables|/Script/CharmTunnelSim.ProceduralTunnel|SetnumberOfVerticalPoints NewParam (Variables|Default|GetnumberOfVerticalPoints)))
    (:then_2
      (Variables|/Script/CharmTunnelSim.ProceduralTunnel|SetloopAroundTunnelLastIndex NewParam (+ (* (Variables|/Script/CharmTunnelSim.ProceduralTunnel|GetnumberOfHorizontalPoints NewParam) 2) (* (Variables|/Script/CharmTunnelSim.ProceduralTunnel|GetnumberOfVerticalPoints NewParam) 2) -1)))))