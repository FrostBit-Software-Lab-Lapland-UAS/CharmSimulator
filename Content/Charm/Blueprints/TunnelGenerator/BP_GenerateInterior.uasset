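; Interior generator that, in simulation mode, dresses every BP_ProceduralTunnel with rock splines and light railings shortly after BeginPlay.
; For each tunnel it spawns left and right BP_RockSpline actors, plus a BP_RailingSpline for longer tunnels.
; It steps along the tunnel spline, placing rock points at width-based side offsets and railing points where rightward traces hit the tunnel wall.
; It then builds the splines and adds the lights, which ClearLights can remove.
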(event Custom|AddLights)

(event Custom|ClearLights
  (for _array_element (Variables|Default|GetLightRailings)
    (Default|RemoveLights _array_element)))

(event EventBeginPlay
  (bind _asrosintegration_game_instance (Utilities|Casting|CastToROSIntegrationGameInstance (Game|GetGameInstance)))
  (if (Variables|/Script/ROSIntegration.ROSIntegrationGameInstance|GetisSimulating _asrosintegration_game_instance)
    (Utilities|FlowControl|Delay 0.2)
    (CallFunction|SpawnInteriors)))

(fn ConstructionScript)

(fn SpawnInteriors
  (bind _spawnedlightspline (Variables|Default|GetSpawnedLightSpline))
  (bind _lightspline (LocalVariables|GetLightSpline))
  (bind _rightrockspline (LocalVariables|GetRightRockSpline))
  (bind _leftrockspline (LocalVariables|GetLeftRockSpline))
  (bind _spline (Variables|/Game/Charm/Blueprints/Props/BP_RockSpline.BP_RockSpline_C|GetSpline _leftrockspline))
  (bind _spline_2 (Variables|/Game/Charm/Blueprints/Props/BP_RockSpline.BP_RockSpline_C|GetSpline _rightrockspline))
  (bind _spline_3 (Variables|/Game/Charm/Blueprints/Props/BP_RailingSpline.BP_RailingSpline_C|GetSpline _lightspline))
  (bind _outactors (Actor|GetAllActorsOfClass "/Game/Charm/Blueprints/TunnelGenerator/BP_ProceduralTunnel.BP_ProceduralTunnel_C"))
  (for _array_element _outactors
    (LocalVariables|SetCurrentTunnel _array_element)
    (Variables|Default|SetDistanceOnSpline 2e+02)
    (|SpawnSplineActors_2)
    (for _index (range 0 (Math|Float|Round (/ (- (Spline|GetSplineLength (Variables|/Script/CharmTunnelSim.ProceduralTunnel|GetSplineComponent (LocalVariables|GetCurrentTunnel))) 2e+02) (Variables|Default|GetDistanceJumpOnSpline))))
      (if (< _index 2)
        (Spline|SetLocationatSplinePoint _spline _index (.LeftSplineLocation (CallFunction|GetRockSplinesPointLocations (LocalVariables|GetCurrentTunnel))) "World" true)
        (Spline|SetLocationatSplinePoint _spline_2 _index (.RightSplineLocation (CallFunction|GetRockSplinesPointLocations (LocalVariables|GetCurrentTunnel))) "World" true)
        (if (.DidHit (CallFunction|GetLineTraceLocation (LocalVariables|GetCurrentTunnel)))
          (if _spawnedlightspline
            (Spline|SetLocationatSplinePoint _spline_3 _index (.HitLocation (CallFunction|GetLineTraceLocation (LocalVariables|GetCurrentTunnel))) "World" true))
          (Variables|Default|SetDistanceOnSpline (Math|Float|SelectFloat (+ (Variables|Default|GetDistanceOnSpline) (Variables|Default|GetDistanceJumpOnSpline)) (Spline|GetSplineLength (Variables|/Script/CharmTunnelSim.ProceduralTunnel|GetSplineComponent (LocalVariables|GetCurrentTunnel))) (< (+ (Variables|Default|GetDistanceOnSpline) (Variables|Default|GetDistanceJumpOnSpline)) (Spline|GetSplineLength (Variables|/Script/CharmTunnelSim.ProceduralTunnel|GetSplineComponent (LocalVariables|GetCurrentTunnel))))) :!label _label))
        (else
          (Spline|AddSplinePoint _spline (.LeftSplineLocation (CallFunction|GetRockSplinesPointLocations (LocalVariables|GetCurrentTunnel))) "World" true)
          (Spline|AddSplinePoint _spline_2 (.RightSplineLocation (CallFunction|GetRockSplinesPointLocations (LocalVariables|GetCurrentTunnel))) "World" true)
          (if (.DidHit (CallFunction|GetLineTraceLocation (LocalVariables|GetCurrentTunnel)))
            (if _spawnedlightspline
              (Spline|AddSplinePoint _spline_3 (.HitLocation (CallFunction|GetLineTraceLocation (LocalVariables|GetCurrentTunnel))) "World" true)
              (goto _label)
              (else
                (goto _label)))))))
    (if (Variables|Default|GetSpawnedLightSpline)
      (Default|ManualConst (LocalVariables|GetLightSpline))))
  (Utilities|FlowControl|Sequence
    (:then_0
      (for _array_element_2 (Variables|Default|GetLightRailings)
        (Default|AddLights _array_element_2)))
    (:then_1
      (for _array_element_3 (Variables|Default|GetRightRockSplines)
        (Default|ManualConst _array_element_3)))
    (:then_2
      (for _array_element_4 (Variables|Default|GetLeftRockSplines)
        (Default|ManualConst _array_element_4)))))

(fn GetLineTraceStartandEnd
  (params (Tunnel :type BP%20Procedural%20Tunnel%20Object%20Reference))
  (bind _verticalpointsize (Variables|/Script/CharmTunnelSim.ProceduralTunnel|GetverticalPointSize Tunnel))
  (bind _height (Variables|/Game/Charm/Blueprints/TunnelGenerator/BP_ProceduralTunnel.BP_ProceduralTunnel_C|GetHeight Tunnel))
  (bind _splinecomponent (Variables|/Script/CharmTunnelSim.ProceduralTunnel|GetSplineComponent Tunnel))
  (bind _distanceonspline (Variables|Default|GetDistanceOnSpline))
  (bind _returnvalue (Spline|GetLocationatDistanceAlongSpline _splinecomponent _distanceonspline "World"))
  (bind _returnvalue_2 (Math|Conversions|ToFloat(Integer) _height))
  (bind _returnvalue_3 (- _returnvalue_2 5.0))
  (bind _returnvalue_4 (* _verticalpointsize _returnvalue_3))
  (bind _returnvalue_5 (+ _returnvalue (Math|Vector|MakeVector 0.0 0.0 _returnvalue_4)))
  (return _returnvalue_5 (+ _returnvalue_5 (* (Class|SplineComponent|GetRightVectoratDistanceAlongSpline _splinecomponent _distanceonspline "World") 1e+03))))

(fn GetRockSplinesPointLocations
  (params (Tunnel :type BP%20Procedural%20Tunnel%20Object%20Reference))
  (bind _horizontalpointsize (Variables|/Script/CharmTunnelSim.ProceduralTunnel|GethorizontalPointSize Tunnel))
  (bind _splinecomponent (Variables|/Script/CharmTunnelSim.ProceduralTunnel|GetSplineComponent Tunnel))
  (bind _distanceonspline (Variables|Default|GetDistanceOnSpline))
  (bind _width (Variables|/Game/Charm/Blueprints/TunnelGenerator/BP_ProceduralTunnel.BP_ProceduralTunnel_C|GetWidth Tunnel))
  (bind _returnvalue (Math|Conversions|ToFloat(Integer) _width))
  (bind _returnvalue_2 (Spline|GetLocationatDistanceAlongSpline _splinecomponent _distanceonspline "World"))
  (bind _returnvalue_3 (Class|SplineComponent|GetRightVectoratDistanceAlongSpline _splinecomponent _distanceonspline "World"))
  (bind _returnvalue_4 (- _returnvalue 12.0))
  (bind _returnvalue_5 (* _horizontalpointsize _returnvalue_4))
  (return (+ _returnvalue_2 (* _returnvalue_3 _returnvalue_5)) (+ _returnvalue_2 (* (* _returnvalue_3 -1.0) _returnvalue_5))))

(fn GetLineTraceLocation
  (params (Tunnel :type BP%20Procedural%20Tunnel%20Object%20Reference))
  (bind (_linetracestart _linetraceend) (CallFunction|GetLineTraceStartandEnd Tunnel))
  (bind _outhit (Collision|LineTraceByChannel _linetracestart _linetraceend "TraceTypeQuery1" false 0 "None"))
  (return (and (.bBlockingHit (Collision|BreakHitResult _outhit)) (== (.HitActor (Collision|BreakHitResult _outhit)) Tunnel)) (+ (.ImpactPoint (Collision|BreakHitResult _outhit)) (* (.ImpactNormal (Collision|BreakHitResult _outhit)) 2e+01))))