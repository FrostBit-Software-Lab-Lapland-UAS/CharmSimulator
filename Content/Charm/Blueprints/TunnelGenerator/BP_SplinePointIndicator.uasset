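; Spline point marker actor for the tunnel generator, shown as a cube or, when IsSphereMesh is set, a sphere with a moving-actor spline point material applied at BeginPlay.
; Enable and Disable toggle the ZArrow's visibility and tint the mesh green or red through its BaseColor material parameter.
; The construction script aligns ZArrow to the mesh in world X and Y, while its spline mesh creation and vertex painting nodes never run.
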(event Custom|Disable
  (Rendering|SetVisibility (Variables|Default|GetZArrow) false false)
  (Rendering|Material|SetVectorParameterValueonMaterials (Variables|Default|GetCube) "BaseColor" "1.000000,0.000000, 0"))

(event Custom|Enable
  (Rendering|SetVisibility (Variables|Default|GetZArrow) true false)
  (Rendering|Material|SetVectorParameterValueonMaterials (Variables|Default|GetCube) "BaseColor" "0,1.000000, 0"))

(event EventBeginPlay
  (if (Variables|Default|GetisSphereMesh)
    (Components|StaticMesh|SetStaticMesh (Variables|Default|GetCube) "/Engine/BasicShapes/Sphere.Sphere")
    (Rendering|Material|SetMaterial (Variables|Default|GetCube) 0 "/Game/Charm/Materials/EventManager/M_MovingActorSplinePoint.M_MovingActorSplinePoint")))

(fn ConstructionScript
  (bind _zarrow (Variables|Default|GetZArrow))
  (bind _cube (Variables|Default|GetCube))
  (bind _returnvalue (Transformation|GetWorldLocation _cube))
  (Transformation|SetWorldLocation _zarrow (Math|Vector|MakeVector (.x _returnvalue) (.y _returnvalue) (.z (Transformation|GetWorldLocation _zarrow))) false false))