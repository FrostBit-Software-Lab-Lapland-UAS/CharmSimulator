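; BP_RockSpline is a prop that scatters instanced meshes, presumably rocks, along a spline.
; The ManualConst event, rather than the empty construction script, walks the spline at Step intervals, adding a world-space instance to one of five randomly picked instanced mesh components.
; Instance rotation and scale come from RotatorAndScale, whose random rotator and scale nodes appear unconnected in its graph.
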(event Custom|ManualConst
  (bind (_rotator _scale) (|RotatorAndScale))
  (bind _step (Variables|Default|GetStep))
  (bind _instancedstaticmesh3 (Variables|Default|GetInstancedStaticMesh3))
  (bind _instancedstaticmesh2 (Variables|Default|GetInstancedStaticMesh2))
  (bind _instancedstaticmesh4 (Variables|Default|GetInstancedStaticMesh4))
  (bind _instancedstaticmesh (Variables|Default|GetInstancedStaticMesh))
  (bind _instancedstaticmesh1 (Variables|Default|GetInstancedStaticMesh1))
  (bind _array (Utilities|Array|MakeArray _instancedstaticmesh4 _instancedstaticmesh _instancedstaticmesh1 _instancedstaticmesh3 _instancedstaticmesh2))
  (for _index (range 0 (Math|Float|Truncate (/ (Spline|GetSplineLength (Variables|Default|GetSpline)) _step)))
    (Class|InstancedStaticMeshComponent|AddInstanceWorldSpace (Utilities|Array|Get(acopy) _array (Math|Random|RandomInteger (Utilities|Array|Length _array))) (Math|Transform|MakeTransform (Spline|GetLocationatDistanceAlongSpline (Variables|Default|GetSpline) (* _index _step) "World") _rotator _scale))))

(event EventBeginPlay)

(event Collision|EventActorBeginOverlap
  (params (OtherActor :type Actor%20Object%20Reference)))

(event EventTick
  (params (DeltaSeconds :type Float%20%28single-precision%29)))

(fn ConstructionScript)