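; BP_PropActor is a configurable prop actor whose static mesh is chosen by a PropType value: rock, metal barrel, plastic drum or traffic cone.
; On BeginPlay it sets that mesh and applies the SimulatePhysics flag to the component.
; A ChangeMesh event swaps the mesh from a passed-in type using the same selection.
; The Random option has no mesh assigned, and the construction script is empty.
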(event Custom|ChangeMesh
  (params (PropType :type PropType%20Enum :default "NewEnumerator0"))
  (Components|StaticMesh|SetStaticMesh (Variables|Default|GetStaticMesh) (Utilities|Select :Index PropType :NewEnumerator0 "/Game/Charm/Meshes/Props/stone5_Cube.stone5_Cube" :NewEnumerator1 "/Game/Megascans/3D_Assets/Rusty_Metal_Barrel_vijnbjz/S_Rusty_Metal_Barrel_vijnbjz_lod3_Var1.S_Rusty_Metal_Barrel_vijnbjz_lod3_Var1" :NewEnumerator2 "/Game/Megascans/3D_Assets/Dirty_Plastic_Drum_uiujbcxva/S_Dirty_Plastic_Drum_uiujbcxva_lod3_Var1.S_Dirty_Plastic_Drum_uiujbcxva_lod3_Var1" :NewEnumerator3 "/Game/Megascans/3D_Assets/Traffic_Cone_vgkwebl/S_Traffic_Cone_vgkwebl_lod3.S_Traffic_Cone_vgkwebl_lod3" :NewEnumerator6 0)))

(event EventBeginPlay
  (Components|StaticMesh|SetStaticMesh (Variables|Default|GetStaticMesh) (Utilities|Select :Index (Variables|Default|GetPropType) :NewEnumerator0 "/Game/Charm/Meshes/Props/stone5_Cube.stone5_Cube" :NewEnumerator1 "/Game/Megascans/3D_Assets/Rusty_Metal_Barrel_vijnbjz/S_Rusty_Metal_Barrel_vijnbjz_lod3_Var1.S_Rusty_Metal_Barrel_vijnbjz_lod3_Var1" :NewEnumerator2 "/Game/Megascans/3D_Assets/Dirty_Plastic_Drum_uiujbcxva/S_Dirty_Plastic_Drum_uiujbcxva_lod3_Var1.S_Dirty_Plastic_Drum_uiujbcxva_lod3_Var1" :NewEnumerator3 "/Game/Megascans/3D_Assets/Traffic_Cone_vgkwebl/S_Traffic_Cone_vgkwebl_lod3.S_Traffic_Cone_vgkwebl_lod3" :NewEnumerator6 0))
  (Physics|SetSimulatePhysics (Variables|Default|GetStaticMesh) (Variables|Default|GetSimulatePhysics)))

(fn ConstructionScript)