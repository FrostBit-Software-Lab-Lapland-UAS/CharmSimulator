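; Railing prop that builds itself along a spline from repeated spline mesh segments and can line it with rail lights.
; The construction script calls ManualConst, which adds one segment per SectionLenght, clamping tangents to that length so the mesh follows the curve.
; AddLights spawns BP_RailLight actors every LightCap units, offset sideways, with the first nudged forward, and tracks them in MineLights.
; RemoveLights destroys those tracked actors; neither light function is called within this Blueprint.
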(event Custom|ManualConst
  (bind _spline (Variables|Default|GetSpline))
  (bind _sectionlenght (Variables|Default|GetSectionLenght))
  (bind _spline_2 (Variables|Default|GetSpline))
  (bind _sectionlenght_2 (Variables|Default|GetSectionLenght))
  (for _index (range 0 (Math|Float|Truncate (/ (Spline|GetSplineLength (Variables|Default|GetSpline)) (Variables|Default|GetSectionLenght))))
    (bind _returnvalue (AddComponent|AddSplineMeshComponent false))
    (SplineMesh|SetStartandEnd _returnvalue (Spline|GetLocationatDistanceAlongSpline _spline_2 (* _index _sectionlenght_2) "Local") (Math|Vector|ClampVectorSize (Spline|GetTangentatDistanceAlongSpline _spline_2 (* _index _sectionlenght_2) "Local") 0.0 _sectionlenght) (Spline|GetLocationatDistanceAlongSpline _spline (* (+ _index 1) _sectionlenght_2) "Local") (Math|Vector|ClampVectorSize (Spline|GetTangentatDistanceAlongSpline _spline (* (+ _index 1) _sectionlenght_2) "Local") 0.0 _sectionlenght) true :!class /Script/Engine.SplineMeshComponent)))

(fn ConstructionScript
  (CallFunction|ManualConst))

(fn AddLights
  (bind _lightcap (Variables|Default|GetLightCap))
  (bind _spline (Variables|Default|GetSpline))
  (for _index (range 0 (Math|Float|Truncate (/ (Spline|GetSplineLength (Variables|Default|GetSpline)) _lightcap)))
    (bind _returnvalue (Game|SpawnActorfromClass "/Game/Charm/Blueprints/Props/BP_RailLight.BP_RailLight_C" (Math|Transform|MakeTransform (+ (+ (Spline|GetLocationatDistanceAlongSpline _spline (* _index _lightcap) "World") (* (Class|SplineComponent|GetRightVectoratDistanceAlongSpline _spline (* _index _lightcap) "World") -15.0)) (Math|Vector|SelectVector (* (Spline|GetDirectionatDistanceAlongSpline _spline (* _index _lightcap) "World") 5e+01) "0, 0, 0" (== _index 0))) (Spline|GetRotationatDistanceAlongSpline _spline (* _index _lightcap) "World") "1.000000,1.000000,1.000000") "Undefined" 0 0))
    (Utilities|Array|Add (Variables|Default|GetMineLights) _returnvalue)))

(fn RemoveLights
  (for _array_element (Variables|Default|GetMineLights)
    (Actor|DestroyActor _array_element)))