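; Inspection vehicle steered by differential throttle on two rear-wheel movement components, with animated wheels and a spawn-spot mesh showing the chosen sensor.
; When ROS is connected, Vector3 commands set each wheel's throttle or brake, and Tick publishes speed and throttle.
; Once started, it follows an assigned spline using look-ahead heading and distance error; a procedural-tunnel variant exists but is uncalled here.
; Scenario trigger overlaps override wheel friction.
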(event Custom|ChangeSpawnSpotMesh
  (params (NewParam :type ENUM_SelectedSensor%20Enum :default "NewEnumerator0"))
  (bind _spawnspot (Variables|Default|GetSpawnSpot))
  ;[1 0 0.9314 1 30] Change Spawnspot mesh to indicate right sensor
  (Components|StaticMesh|SetStaticMesh _spawnspot (Utilities|Select :Index NewParam :NewEnumerator3 0 :NewEnumerator0 "/Game/Charm/Meshes/Sensors/Ouster_Cylinder_006.Ouster_Cylinder_006" :NewEnumerator1 "/Engine/BasicShapes/Cube.Cube" :NewEnumerator2 "/Game/Charm/Meshes/Sensors/gopro_Cube.gopro_Cube"))
  (Transformation|SetWorldScale3D _spawnspot (Utilities|Select :Index NewParam :NewEnumerator3 "0, 0, 0" :NewEnumerator0 "1.000000,1.000000,1.000000" :NewEnumerator1 "0.039969,0.133799,0.083594" :NewEnumerator2 "1.000000,1.000000,1.000000")))

(event Custom|ReceivedVehicleCommand
  (params (NewParam :type Vector))
  ;[1 0.5063 0 1 30] Get animation blueprint. Create topic for getting vehicle commands. Bind event to subscription and handle input commands of vehicle.
  (CallFunction|GetThrottleValues (.x NewParam) (.y NewParam))
  (Throttle|SetThrottle))

(event EventBeginPlay
  ;[1 0.5063 0 1 30] Get animation blueprint. Create topic for getting vehicle commands. Bind event to subscription and handle input commands of vehicle.
  (Utilities|FlowControl|Delay 1.0)
  (bind _asterttu_anim_blueprint (Utilities|Casting|CastToterttu_AnimBlueprint (Components|SkeletalMesh|GetAnimInstance (Variables|Character|GetMesh))))
  (Variables|Default|SetAs%20Terttu%20Anim%20Blueprint _asterttu_anim_blueprint)
  (bind _asrosintegration_game_instance (Utilities|Casting|CastToROSIntegrationGameInstance (Game|GetGameInstance)))
  (if (Variables|/Script/ROSIntegration.ROSIntegrationGameInstance|GetbIsConnected _asrosintegration_game_instance)
    (bind _returnvalue (Game|ConstructObjectfromClass "/Game/Charm/Blueprints/Topic/BP_TopicManager.BP_TopicManager_C"))
    (bind _output_get (Variables|ROS|SetTopicManager _returnvalue))
    (Default|CreateandSub _output_get "/unreal/vehicle" "Vector3")
    (EventDispatchers|BindEventtoReceivedVectorMessage _output_get (delegate Custom|ReceivedVehicleCommand))
    (bind _returnvalue_2 (Game|ConstructObjectfromClass "/Game/Charm/Blueprints/Topic/BP_TopicManager.BP_TopicManager_C"))
    (bind _output_get_2 (Variables|ROS|SetSpeedTopic _returnvalue_2))
    (Default|CreateandSub _output_get_2 "/unreal/vehicle/speed" "String")
    (bind _returnvalue_3 (Game|ConstructObjectfromClass "/Game/Charm/Blueprints/Topic/BP_TopicManager.BP_TopicManager_C"))
    (bind _output_get_3 (Variables|ROS|SetLeftThrottleTopic _returnvalue_3))
    (Default|CreateandSub _output_get_3 "/unreal/vehicle/leftwheel/throttle" "String")
    (bind _returnvalue_4 (Game|ConstructObjectfromClass "/Game/Charm/Blueprints/Topic/BP_TopicManager.BP_TopicManager_C"))
    (bind _output_get_4 (Variables|ROS|SetRightThrottleTopic _returnvalue_4))
    (Default|CreateandSub _output_get_4 "/unreal/vehicle/rightwheel/throttle" "String")))

(event Collision|EventActorBeginOverlap
  (params (OtherActor :type Actor%20Object%20Reference))
  ;[0.2428 1 0 1 30] Events when entering friction triggers
  (bind _asbp_scenario_trigger (Utilities|Casting|CastToBP_ScenarioTrigger OtherActor))
  (Variables|Default|SetOverlap true)
  (Class|ChaosWheeledVehicleMovementComponent|SetWheelFrictionMultiplier (Variables|Default|GetBackLeftMovementComponent) 0 (Math|Float|SelectFloat (Variables|/Game/Charm/Blueprints/EventSystem/BP_ScenarioActor.BP_ScenarioActor_C|GetFrictionValue _asbp_scenario_trigger) 2.0 (Variables|Default|GetOverlap)))
  (Class|ChaosWheeledVehicleMovementComponent|SetWheelFrictionMultiplier (Variables|Default|GetBackRightMovementComponent) 0 (Math|Float|SelectFloat (Variables|/Game/Charm/Blueprints/EventSystem/BP_ScenarioActor.BP_ScenarioActor_C|GetFrictionValue _asbp_scenario_trigger) 2.0 (Variables|Default|GetOverlap))))

(event Collision|EventActorEndOverlap
  (params (OtherActor :type Actor%20Object%20Reference))
  ;[0.2428 1 0 1 30] Events when entering friction triggers
  (Utilities|Casting|CastToBP_ScenarioTrigger OtherActor)
  (Variables|Default|SetOverlap false)
  (Class|ChaosWheeledVehicleMovementComponent|SetWheelFrictionMultiplier (Variables|Default|GetBackLeftMovementComponent) 0 (Math|Float|SelectFloat (Variables|/Game/Charm/Blueprints/EventSystem/BP_ScenarioActor.BP_ScenarioActor_C|GetFrictionValue (stale Collision|EventActorBeginOverlap _asbp_scenario_trigger)) 2.0 (Variables|Default|GetOverlap)))
  (Class|ChaosWheeledVehicleMovementComponent|SetWheelFrictionMultiplier (Variables|Default|GetBackRightMovementComponent) 0 (Math|Float|SelectFloat (Variables|/Game/Charm/Blueprints/EventSystem/BP_ScenarioActor.BP_ScenarioActor_C|GetFrictionValue (stale Collision|EventActorBeginOverlap _asbp_scenario_trigger)) 2.0 (Variables|Default|GetOverlap))))

(event EventEndPlay
  (params (EndPlayReason :type EEndPlayReason%20Enum :default "Destroyed"))
  (Actor|Tick|SetActorTickEnabled false)
  (Variables|ROS|SetSpeedTopic 0)
  (Variables|ROS|SetLeftThrottleTopic 0)
  (Variables|ROS|SetRightThrottleTopic 0)
  (Variables|ROS|SetTopicManager 0))

(event EventTick
  (params (DeltaSeconds :type Float%20%28single-precision%29))
  (bind _as_terttu_anim_blueprint (Variables|Default|GetAs%20Terttu%20Anim%20Blueprint))
  (bind _speedtopic (Variables|ROS|GetSpeedTopic))
  ;[1 0 0.05342 1 30] Animate vehicle back wheels
  (Utilities|FlowControl|Sequence
    (:then_0
      (Variables|Default|SetDelta%20Seconds DeltaSeconds)
      (if (Utilities|IsValid (Variables|Default|GetAs%20Terttu%20Anim%20Blueprint))
        (Variables|/Game/Charm/Blueprints/Vehicle/terttu_AnimBlueprint.terttu_AnimBlueprint_C|SetRightWheelSpeed _as_terttu_anim_blueprint (|RightWheel))
        (Variables|/Game/Charm/Blueprints/Vehicle/terttu_AnimBlueprint.terttu_AnimBlueprint_C|SetLeftWheelSpeed _as_terttu_anim_blueprint (|LeftWheel))
        (if (Variables|Default|GetisStarted)
          (Utilities|IsValid (Variables|Default|GetSplineToFollow)
            (:Is%20Valid
              (CallFunction|FollowSpineinScannedTunnel))))))
    (:then_1
      (Utilities|IsValid _speedtopic
        (:Is%20Valid
          (Class|Topic|PublishStringMessage _speedtopic (Utilities|String|ToString(Float) (* (Class|ChaosVehicleMovementComponent|GetForwardSpeedMPH (Variables|Default|GetBackLeftMovementComponent)) 1.60934))))
        (:Is%20Not%20Valid
          _))
      (Utilities|IsValid (Variables|ROS|GetLeftThrottleTopic)
        (:Is%20Valid
          (bind _returnvalue (Class|ChaosVehicleMovementComponent|GetThrottleInput (Variables|Default|GetBackLeftMovementComponent)))
          (Class|Topic|PublishStringMessage (Variables|ROS|GetLeftThrottleTopic) (Utilities|String|ToString(Float) _returnvalue)))
        (:Is%20Not%20Valid
          _))
      (Utilities|IsValid (Variables|ROS|GetRightThrottleTopic)
        (:Is%20Valid
          (bind _returnvalue_2 (Class|ChaosVehicleMovementComponent|GetThrottleInput (Variables|Default|GetBackRightMovementComponent)))
          (Class|Topic|PublishStringMessage (Variables|ROS|GetRightThrottleTopic) (Utilities|String|ToString(Float) _returnvalue_2)))))))

(fn ConstructionScript)

(fn ManualThrottle
  (Utilities|FlowControl|Sequence
    (:then_0
      (Class|ChaosVehicleMovementComponent|SetThrottleInput (Variables|Default|GetBackRightMovementComponent) (Math|Float|SelectFloat 0.0 1.0 (== (Variables|Throttle|GetBackRightWheelThrottle) 0.0))))
    (:then_1
      (Class|ChaosVehicleMovementComponent|SetThrottleInput (Variables|Default|GetBackLeftMovementComponent) (Math|Float|SelectFloat 0.0 1.0 (== (Variables|Throttle|GetBackLeftWheelThrottle) 0.0))))))

(fn SetThrottle
  (bind _backrightmovementcomponent (Variables|Default|GetBackRightMovementComponent))
  (bind _backrightmovementcomponent_2 (Variables|Default|GetBackRightMovementComponent))
  (bind _backleftwheelthrottle (Variables|Throttle|GetBackLeftWheelThrottle))
  (bind _backleftmovementcomponent (Variables|Default|GetBackLeftMovementComponent))
  (Utilities|FlowControl|Sequence
    (:then_0
      (if (< (Variables|Throttle|GetBackRightWheelThrottle) 0.0)
        (Class|ChaosVehicleMovementComponent|SetThrottleInput _backrightmovementcomponent_2 0.0)
        (Class|ChaosVehicleMovementComponent|SetBrakeInput _backrightmovementcomponent_2 (Math|Float|Absolute(Float) (Variables|Throttle|GetBackRightWheelThrottle)))
        (else
          (Class|ChaosVehicleMovementComponent|SetThrottleInput _backrightmovementcomponent (Variables|Throttle|GetBackRightWheelThrottle))
          (Class|ChaosVehicleMovementComponent|SetBrakeInput _backrightmovementcomponent 0.0))))
    (:then_1
      (if (< (Variables|Throttle|GetBackLeftWheelThrottle) 0.0)
        (Class|ChaosVehicleMovementComponent|SetThrottleInput _backleftmovementcomponent 0.0)
        (Class|ChaosVehicleMovementComponent|SetBrakeInput _backleftmovementcomponent (Math|Float|Absolute(Float) _backleftwheelthrottle))
        (else
          (Class|ChaosVehicleMovementComponent|SetThrottleInput _backleftmovementcomponent _backleftwheelthrottle)
          (Class|ChaosVehicleMovementComponent|SetBrakeInput _backleftmovementcomponent 0.0))))))

(fn SetBrakes
  (Utilities|FlowControl|Sequence
    (:then_0
      (Class|ChaosVehicleMovementComponent|SetBrakeInput (Variables|Default|GetBackRightMovementComponent) (Math|Float|SelectFloat 0.5 0.0 (>= (* (Vehicle|GetForwardSpeed (Variables|Default|GetBackRightMovementComponent)) 0.036) (Math|Float|Lerp 1.0 1e+01 (Variables|Throttle|GetBackRightWheelThrottle))))))
    (:then_1
      (Class|ChaosVehicleMovementComponent|SetBrakeInput (Variables|Default|GetBackLeftMovementComponent) (Math|Float|SelectFloat 0.5 0.0 (>= (* (Vehicle|GetForwardSpeed (Variables|Default|GetBackLeftMovementComponent)) 0.036) (Math|Float|Lerp 1.0 1e+01 (Variables|Throttle|GetBackLeftWheelThrottle))))))))

(fn FollowSpineinScannedTunnel
  (bind _returnvalue (Transformation|GetActorLocation))
  (bind _returnvalue_2 (Transformation|GetActorRotation))
  (bind _returnvalue_3 (Transformation|GetActorLocation))
  (bind _splinetofollow (Variables|Default|GetSplineToFollow))
  (bind _mesh (Variables|Character|GetMesh))
  (bind _splinetofollow_2 (Variables|Default|GetSplineToFollow))
  (bind _maxspeedinfakedrive (Variables|Default|GetMaxSpeedInFakeDrive))
  (bind _backleftmovementcomponent (Variables|Default|GetBackLeftMovementComponent))
  (bind _returnvalue_4 (Math|Vector|GetForwardVector _mesh))
  (bind _returnvalue_5 (Class|ChaosVehicleMovementComponent|GetForwardSpeedMPH _backleftmovementcomponent))
  (bind _spline (Variables|/Game/Charm/Blueprints/EventSystem/BP_MovingObjectEvent.BP_MovingObjectEvent_C|GetSpline _splinetofollow_2))
  (bind _spline_2 (Variables|/Game/Charm/Blueprints/EventSystem/BP_MovingObjectEvent.BP_MovingObjectEvent_C|GetSpline _splinetofollow))
  (bind _returnvalue_6 (Class|SplineComponent|FindInputKeyClosesttoWorldLocation _spline_2 _returnvalue))
  (bind _returnvalue_7 (Spline|FindLocationClosesttoWorldLocation _spline _returnvalue_3 "World"))
  (bind _returnvalue_8 (Spline|FindDirectionClosesttoWorldLocation _spline_2 _returnvalue "World"))
  (bind _returnvalue_9 (> _returnvalue_5 5.0))
  (bind _returnvalue_10 (Math|Float|SelectFloat 0.0 _maxspeedinfakedrive _returnvalue_9))
  (bind _returnvalue_11 (Class|SplineComponent|GetDistanceAlongSplineatSplineInputKey _spline_2 _returnvalue_6))
  (bind _returnvalue_12 (Math|Vector|Distance(Vector) _returnvalue_3 _returnvalue_7))
  (bind _returnvalue_13 (Math|Vector|DotProduct _returnvalue_4 _returnvalue_8))
  (bind _returnvalue_14 (Math|Float|Clamp(Float) _returnvalue_12 0.0 1e+02))
  (bind _returnvalue_15 (/ _returnvalue_10 2.0))
  (bind _returnvalue_16 (< _returnvalue_13 0.0))
  (bind _returnvalue_17 (Math|Float|NormalizetoRange _returnvalue_14 0.0 1e+02))
  (bind _returnvalue_18 (Math|Float|SelectFloat -5e+02 5e+02 _returnvalue_16))
  (bind _returnvalue_19 (+ _returnvalue_11 _returnvalue_18))
  (bind _returnvalue_20 (Spline|GetLocationatDistanceAlongSpline _spline_2 _returnvalue_19 "World"))
  (bind _returnvalue_21 (Math|Rotator|FindLookatRotation _returnvalue _returnvalue_20))
  (bind _returnvalue_22 (Math|Rotator|Delta(Rotator) _returnvalue_2 _returnvalue_21))
  (bind _returnvalue_23 (Math|Float|Clamp(Float) (.yaw _returnvalue_22) -1.8e+02 1.8e+02))
  (bind _returnvalue_24 (< (.yaw _returnvalue_22) 0.0))
  (bind _returnvalue_25 (/ _returnvalue_23 1.8e+02))
  (bind _returnvalue_26 (Math|Float|Absolute(Float) _returnvalue_25))
  (bind _returnvalue_27 (+ _returnvalue_17 _returnvalue_26))
  (bind _returnvalue_28 (/ _returnvalue_27 2.0))
  (bind _returnvalue_29 (Math|Float|Lerp _returnvalue_15 0.0 _returnvalue_28))
  (Class|ChaosVehicleMovementComponent|SetThrottleInput (Variables|Default|GetBackLeftMovementComponent) (Math|Float|SelectFloat _returnvalue_10 _returnvalue_29 _returnvalue_24))
  (Class|ChaosVehicleMovementComponent|SetThrottleInput (Variables|Default|GetBackRightMovementComponent) (Math|Float|SelectFloat _returnvalue_29 _returnvalue_10 _returnvalue_24)))

(fn FollowSplineinCreatedTunnel
  (bind _returnvalue (Transformation|GetActorLocation))
  (bind _returnvalue_2 (Transformation|GetActorLocation))
  (bind _returnvalue_3 (Transformation|GetActorLocation))
  (bind _mesh (Variables|Character|GetMesh))
  (bind _returnvalue_4 (Math|Vector|GetForwardVector _mesh))
  (bind _returnvalue_5 (* _returnvalue_4 5e+02))
  (bind _returnvalue_6 (+ _returnvalue_2 _returnvalue_5))
  (bind _returnvalue_7 (+ _returnvalue_6 "0.000000,0.000000,20.000000"))
  (bind _outhit (Collision|LineTraceByChannel _returnvalue_7 (- _returnvalue_7 "0.000000,0.000000,500.000000") "TraceTypeQuery1" false 0 "None"))
  (bind _asbp_procedural_tunnel (Utilities|Casting|CastToBP_ProceduralTunnel (.HitActor (Collision|BreakHitResult _outhit)))
    (:then
      (Variables|Default|SetTunnelToFollow _asbp_procedural_tunnel)
      (Class|ChaosVehicleMovementComponent|SetThrottleInput (Variables|Default|GetBackLeftMovementComponent) (Math|Float|SelectFloat 0.25 (Math|Float|Lerp 0.25 0.1 (/ (+ (Math|Float|NormalizetoRange (Math|Float|Clamp(Float) (Math|Vector|Distance(Vector) _returnvalue_3 (Spline|FindLocationClosesttoWorldLocation (Variables|/Script/CharmTunnelSim.ProceduralTunnel|GetSplineComponent (Variables|Default|GetTunnelToFollow)) _returnvalue_3 "World")) 0.0 1e+02) 0.0 1e+02) (Math|Float|Absolute(Float) (/ (Math|Float|Clamp(Float) (.yaw (Math|Rotator|Delta(Rotator) (Transformation|GetActorRotation) (Math|Rotator|FindLookatRotation _returnvalue (Spline|GetLocationatDistanceAlongSpline (Variables|/Script/CharmTunnelSim.ProceduralTunnel|GetSplineComponent (Variables|Default|GetTunnelToFollow)) (+ (Class|SplineComponent|GetDistanceAlongSplineatSplineInputKey (Variables|/Script/CharmTunnelSim.ProceduralTunnel|GetSplineComponent (Variables|Default|GetTunnelToFollow)) (Class|SplineComponent|FindInputKeyClosesttoWorldLocation (Variables|/Script/CharmTunnelSim.ProceduralTunnel|GetSplineComponent (Variables|Default|GetTunnelToFollow)) _returnvalue)) (Math|Float|SelectFloat -5e+02 5e+02 (< (Math|Vector|DotProduct (Math|Vector|GetForwardVector (Variables|Character|GetMesh)) (Spline|FindDirectionClosesttoWorldLocation (Variables|/Script/CharmTunnelSim.ProceduralTunnel|GetSplineComponent (Variables|Default|GetTunnelToFollow)) _returnvalue_7 "Local")) 0.0))) "World")))) -9e+01 9e+01) 9e+01))) 2.0)) (< (.yaw (Math|Rotator|Delta(Rotator) (Transformation|GetActorRotation) (Math|Rotator|FindLookatRotation _returnvalue (Spline|GetLocationatDistanceAlongSpline (Variables|/Script/CharmTunnelSim.ProceduralTunnel|GetSplineComponent (Variables|Default|GetTunnelToFollow)) (+ (Class|SplineComponent|GetDistanceAlongSplineatSplineInputKey (Variables|/Script/CharmTunnelSim.ProceduralTunnel|GetSplineComponent (Variables|Default|GetTunnelToFollow)) (Class|SplineComponent|FindInputKeyClosesttoWorldLocation (Variables|/Script/CharmTunnelSim.ProceduralTunnel|GetSplineComponent (Variables|Default|GetTunnelToFollow)) _returnvalue)) (Math|Float|SelectFloat -5e+02 5e+02 (< (Math|Vector|DotProduct (Math|Vector|GetForwardVector (Variables|Character|GetMesh)) (Spline|FindDirectionClosesttoWorldLocation (Variables|/Script/CharmTunnelSim.ProceduralTunnel|GetSplineComponent (Variables|Default|GetTunnelToFollow)) _returnvalue_7 "Local")) 0.0))) "World")))) 0.0)))
      (Class|ChaosVehicleMovementComponent|SetThrottleInput (Variables|Default|GetBackRightMovementComponent) (Math|Float|SelectFloat (Math|Float|Lerp 0.25 0.1 (/ (+ (Math|Float|NormalizetoRange (Math|Float|Clamp(Float) (Math|Vector|Distance(Vector) _returnvalue_3 (Spline|FindLocationClosesttoWorldLocation (Variables|/Script/CharmTunnelSim.ProceduralTunnel|GetSplineComponent (Variables|Default|GetTunnelToFollow)) _returnvalue_3 "World")) 0.0 1e+02) 0.0 1e+02) (Math|Float|Absolute(Float) (/ (Math|Float|Clamp(Float) (.yaw (Math|Rotator|Delta(Rotator) (Transformation|GetActorRotation) (Math|Rotator|FindLookatRotation _returnvalue (Spline|GetLocationatDistanceAlongSpline (Variables|/Script/CharmTunnelSim.ProceduralTunnel|GetSplineComponent (Variables|Default|GetTunnelToFollow)) (+ (Class|SplineComponent|GetDistanceAlongSplineatSplineInputKey (Variables|/Script/CharmTunnelSim.ProceduralTunnel|GetSplineComponent (Variables|Default|GetTunnelToFollow)) (Class|SplineComponent|FindInputKeyClosesttoWorldLocation (Variables|/Script/CharmTunnelSim.ProceduralTunnel|GetSplineComponent (Variables|Default|GetTunnelToFollow)) _returnvalue)) (Math|Float|SelectFloat -5e+02 5e+02 (< (Math|Vector|DotProduct (Math|Vector|GetForwardVector (Variables|Character|GetMesh)) (Spline|FindDirectionClosesttoWorldLocation (Variables|/Script/CharmTunnelSim.ProceduralTunnel|GetSplineComponent (Variables|Default|GetTunnelToFollow)) _returnvalue_7 "Local")) 0.0))) "World")))) -9e+01 9e+01) 9e+01))) 2.0)) 0.25 (< (.yaw (Math|Rotator|Delta(Rotator) (Transformation|GetActorRotation) (Math|Rotator|FindLookatRotation _returnvalue (Spline|GetLocationatDistanceAlongSpline (Variables|/Script/CharmTunnelSim.ProceduralTunnel|GetSplineComponent (Variables|Default|GetTunnelToFollow)) (+ (Class|SplineComponent|GetDistanceAlongSplineatSplineInputKey (Variables|/Script/CharmTunnelSim.ProceduralTunnel|GetSplineComponent (Variables|Default|GetTunnelToFollow)) (Class|SplineComponent|FindInputKeyClosesttoWorldLocation (Variables|/Script/CharmTunnelSim.ProceduralTunnel|GetSplineComponent (Variables|Default|GetTunnelToFollow)) _returnvalue)) (Math|Float|SelectFloat -5e+02 5e+02 (< (Math|Vector|DotProduct (Math|Vector|GetForwardVector (Variables|Character|GetMesh)) (Spline|FindDirectionClosesttoWorldLocation (Variables|/Script/CharmTunnelSim.ProceduralTunnel|GetSplineComponent (Variables|Default|GetTunnelToFollow)) _returnvalue_7 "Local")) 0.0))) "World")))) 0.0))))
    (:CastFailed
      (Class|ChaosVehicleMovementComponent|SetThrottleInput (Variables|Default|GetBackLeftMovementComponent) 0.5)
      (Class|ChaosVehicleMovementComponent|SetThrottleInput (Variables|Default|GetBackRightMovementComponent) 0.5))))

(fn StopVehicle
  (Utilities|FlowControl|Sequence
    (:then_0
      (Class|ChaosVehicleMovementComponent|SetThrottleInput (Variables|Default|GetBackRightMovementComponent) 0.0)
      (Variables|Throttle|SetBackRightWheelThrottle 0.0))
    (:then_1
      (Class|ChaosVehicleMovementComponent|SetThrottleInput (Variables|Default|GetBackLeftMovementComponent) 0.0)
      (Variables|Throttle|SetBackLeftWheelThrottle 0.0))))

(fn GetThrottleValues
  (params (RightWheel :type Float%20%28double-precision%29) (LeftWheel :type Float%20%28double-precision%29))
  (Variables|Throttle|SetBackRightWheelThrottle (Math|Float|SelectFloat 0.0 (* (Math|Float|SelectFloat -1.0 1.0 (< RightWheel 0.0)) (Math|Float|Lerp 0.07 0.5 (Math|Float|Absolute(Float) RightWheel))) (== RightWheel 0.0)))
  (Variables|Throttle|SetBackLeftWheelThrottle (Math|Float|SelectFloat 0.0 (* (Math|Float|SelectFloat -1.0 1.0 (< LeftWheel 0.0)) (Math|Float|Lerp 0.07 0.5 (Math|Float|Absolute(Float) LeftWheel))) (== LeftWheel 0.0))))